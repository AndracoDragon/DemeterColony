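; BP_MenuAnimals is an AI-driven character that keeps an animal wandering, apparently as ambient life for a menu scene.
; On BeginPlay it applies its configured walk speed and starts a Movement event.
; A FlipFlop alternates AI MoveTo between the PlayerStart actor and a random navigable point near the animal's current location.
; Both success and failure call Movement again, so the wandering loops without a delay.
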(event `self.ReceiveBeginPlay`
  (set `CharacterMovementComponent.MaxWalkSpeed` (`self.Max Walk Speed`) (`self.CharacterMovement`))
  (`self.Movement`))

(event `Movement`
  (bind _returnvalue (`AIBlueprintHelperLibrary.GetAIController` self))
  (`/Engine/EditorBlueprintResources/StandardMacros.FlipFlop`
    (:`A`
      (`AITask_MoveTo.AIMoveTo` _returnvalue (-1411.230271 -59.007882 6196.464472) (`self.PlayerStart`)
        (:`OnRequestFailed`
          _)
        (:`OnMoveFinished`
          _)))
    (:`B`
      (bind _randomlocation (`NavigationSystemV1.K2_GetRandomLocationInNavigableRadius` (`self.K2_GetActorLocation`) 3000.0 null null))
      (`AITask_MoveTo.AIMoveTo` _returnvalue _randomlocation null
        (:`OnRequestFailed`
          _)
        (:`OnMoveFinished`
          _))))
  (`self.Movement`))

(fn `UserConstructionScript`)