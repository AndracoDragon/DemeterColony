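; Farm crop actor that grows from a seed's data table row, bears harvestable produce and reports its state as look-at text.
; An Ultra Dynamic Sky hourly event runs growth at hour 2, checking month (only the last listed counts) and soil watering.
; Watered plants jump to full scale, then count up to produce; drought or wrong season kills them.
; Interacting spawns a random item quantity, destroying non-everbearing plants.
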(event `self.ReceiveBeginPlay`
  (bind (_uds _udw) (`/Game/Dynamic/CustomBPS/BlueprintFunctionLibrary.GetUDSandUDW`))
  (set `self.UDW` _udw)
  (set `self.UDS` _uds)
  (`self.InitialPlant`))

(event `InitialPlant`
  (bind _seedwith_ (`self.Seedwith?`))
  (bind _plant (`self.Plant`))
  (bind _returnvalue (`|GetDataTableRow` (break `DataTableRowHandle` (break `/Game/Dynamic/InventorySystem/F_SlotStruct` _seedwith_)) (`.RowName` (break `DataTableRowHandle` (break `/Game/Dynamic/InventorySystem/F_SlotStruct` _seedwith_))))
    (:`then`
      (bind (_datatable _rowname) (break `DataTableRowHandle` (`.Plants_51_5AA2D028465E85CD999D27925A4E92C9` (break `/Game/Dynamic/InventorySystem/F_ItemStruct` _returnvalue))))
      (bind _returnvalue_2 (`|GetDataTableRow` _datatable _rowname)
        (:`then`
          (bind (_name _growthlimit _secondarygrowthlimit _secondarygrowthtimer _producequanitymin _producequanitymax _mainmesh _producemesh _seasonsofgrowth _everbearing_ _everbearingcycle _witherlimit _withertimer _currentgrowth _dead_ _location _unharvested _producetodrop) (break `/Game/Dynamic/CustomBPS/PlantSystem/F_Plants` _returnvalue_2))
          (set `self.PlantStruct` (make `/Game/Dynamic/CustomBPS/PlantSystem/F_Plants` _name _growthlimit _secondarygrowthlimit _secondarygrowthtimer _producequanitymin _producequanitymax _mainmesh _producemesh _seasonsofgrowth _everbearing_ _everbearingcycle _witherlimit _withertimer (0.0 0.0 0.0) false (0.0 0.0 0.0) false _producetodrop))
          (`StaticMeshComponent.SetStaticMesh` _plant _mainmesh)
          (`SceneComponent.SetWorldScale3D` _plant (0.01 0.01 0.01))
          (add `/Game/Dynamic/UltraDynamicSky/Blueprints/Ultra_Dynamic_Sky.Hourly` (`self.UDS`) (delegate `Growth`)))))))

(event `Growth`
  (params (Hour :type Integer))
  (if (`KismetMathLibrary.InRange_IntInt` Hour 2 3 true false)
    (`self.Grow`)))

(event `Grow`
  (bind _plantstruct (`self.PlantStruct`))
  (bind _plantstruct_2 (`self.PlantStruct`))
  (bind _plant (`self.Plant`))
  (bind _plantstruct_3 (`self.PlantStruct`))
  (bind ((`Growthlimit_44_BED62CE4495D0D51962587B070DFFCAB` _growthlimit) (`SecondaryGrowthlimit_50_C47E940D406F37A9EB8251963E139BD5` _secondarygrowthlimit) (`SecondaryGrowthTimer_49_E00A6E284A71DCF4F4A3358682D32152` _secondarygrowthtimer) (`ProduceQuanityMin_58_17E413454D2EA734404DAD905E99C7FD` _producequanitymin) (`ProduceQuanityMax_55_AB8FEEB8413D2F9A8591B4A4AAF8EF36` _producequanitymax) (`MainMesh_32_09ECFF324DB97CD15126C88827A900D5` _mainmesh) (`ProduceMesh_35_676216C247C21C31D4B73281064ECD86` _producemesh) (`WitherLimit_26_50B3CAFD43D196336E2C5FAF72EC55EB` _witherlimit) (`WitherTimer_28_14697DD34F2B3BDBC3376F9D4FF6270F` _withertimer)) (break `/Game/Dynamic/CustomBPS/PlantSystem/F_Plants` _plantstruct_3))
  (bind ((`SecondaryGrowthlimit_50_C47E940D406F37A9EB8251963E139BD5` _secondarygrowthlimit_2) (`SecondaryGrowthTimer_49_E00A6E284A71DCF4F4A3358682D32152` _secondarygrowthtimer_2) (`ProduceQuanityMin_58_17E413454D2EA734404DAD905E99C7FD` _producequanitymin_2) (`ProduceQuanityMax_55_AB8FEEB8413D2F9A8591B4A4AAF8EF36` _producequanitymax_2) (`ProduceMesh_35_676216C247C21C31D4B73281064ECD86` _producemesh_2) (`Everbearing?_17_A6B755E74A843C263D4F3D8E484FDC6F` _everbearing_) (`Unharvested_54_EEE9DA0B4852A2DA49E0209FE17E039A` _unharvested)) (break `/Game/Dynamic/CustomBPS/PlantSystem/F_Plants` (`self.PlantStruct`)))
  (bind _returnvalue (== _secondarygrowthlimit_2 _secondarygrowthtimer_2))
  ;[1 1 1] Plant Code
  ;;[1 1 1] Checks if Dead
  (if (not (`.Dead?_38_D71844C44126D97C2085BBA1CCE7E896` (break `/Game/Dynamic/CustomBPS/PlantSystem/F_Plants` (`self.PlantStruct`))))
    ;;[1 1 1] Checks for Correct Season
    (for _array_element (`.Seasonsofgrowth_22_74657DD14529E459F5F409867581F730` (break `/Game/Dynamic/CustomBPS/PlantSystem/F_Plants` (`self.PlantStruct`)))
      (if (== _array_element (`/Game/Dynamic/UltraDynamicSky/Blueprints/Ultra_Dynamic_Sky.Month` (`self.UDS`)))
        (set `self.RightSeason?` true)
        (else
          (set `self.RightSeason?` false))))
    (if (`self.RightSeason?`)
      ;;[1 1 1] Checks if Watered
      (if (`/Game/Dynamic/CustomBPS/PlantSystem/BP_1TillSoil1.Watered?` (`self.TilledTo?`))
        ;;[1 1 1] Grows Plant
        (setmembers `/Game/Dynamic/CustomBPS/PlantSystem/F_Plants` :`StructRef` _plantstruct_3 :`WitherTimer` 0)
        (if (== (`SceneComponent.K2_GetComponentScale` _plant) (1.0 1.0 1.0) :`ErrorTolerance` 0.1)
          (`SceneComponent.SetWorldScale3D` (`self.Plant`) (1.0 1.0 1.0))
          (if _everbearing_
            ;;[1 1 1] EverbearingFruitCode
            (if (and _returnvalue _unharvested)
              _
              (elif _returnvalue
                (setmembers `/Game/Dynamic/CustomBPS/PlantSystem/F_Plants` :`StructRef` _plantstruct_2 :`Unharvested` true)
                (`StaticMeshComponent.SetStaticMesh` (`self.ProduceMesh`) _producemesh_2)
                (else
                  (setmembers `/Game/Dynamic/CustomBPS/PlantSystem/F_Plants` :`StructRef` _plantstruct_2 :`SecondaryGrowthTimer` (+ _secondarygrowthtimer_2 1)))))
            (else
              ;;[1 1 1] SingularProduceCode
              (if _unharvested
                _
                (elif (== _secondarygrowthlimit_2 _secondarygrowthtimer_2)
                  (bind _structout (setmembers `/Game/Dynamic/CustomBPS/PlantSystem/F_Plants` :`StructRef` _plantstruct :`Unharvested` true))
                  (`StaticMeshComponent.SetStaticMesh` (`self.ProduceMesh`) (`.MainMesh_32_09ECFF324DB97CD15126C88827A900D5` (break `/Game/Dynamic/CustomBPS/PlantSystem/F_Plants` _structout)))
                  (else
                    (setmembers `/Game/Dynamic/CustomBPS/PlantSystem/F_Plants` :`StructRef` _plantstruct :`SecondaryGrowthTimer` (+ _secondarygrowthtimer_2 1)))))))
          (else
            (`SceneComponent.SetWorldScale3D` _plant (1.0 1.0 1.0))
            (setmembers `/Game/Dynamic/CustomBPS/PlantSystem/F_Plants` :`StructRef` (`self.PlantStruct`) :`CurrentGrowth` (1.0 1.0 1.0))))
        (else
          (bind _result (`/Engine/EditorBlueprintResources/StandardMacros.IncrementInt` _withertimer)
            (:`  `
              (setmembers `/Game/Dynamic/CustomBPS/PlantSystem/F_Plants` :`StructRef` _plantstruct_3 :`WitherTimer` _result)
              (if (>= _withertimer _witherlimit)
                (`self.DIE`))))))
      (else
        (`self.DIE`)))))

(event `DIE`
  (bind _plant (`self.Plant`))
  ;[1 1 1] Plant Code
  ;;[1 1 1] Plant Death
  (setmembers `/Game/Dynamic/CustomBPS/PlantSystem/F_Plants` :`StructRef` (`self.PlantStruct`) :`Dead?` true)
  (`StaticMeshComponent.SetStaticMesh` _plant "/Game/Static/Meshes/PlantMeshes/DeadPlant/DeadPlant.DeadPlant")
  (`SceneComponent.SetWorldScale3D` _plant (1.0 1.0 1.0)))

(event `/Game/Dynamic/InventorySystem/I_InteractInterface.InteractWith`
  (params (Player :type "/Game/Dynamic/ThirdPerson/Blueprints/BP_ThirdPersonCharacter Object Reference"))
  (bind (_name _growthlimit _secondarygrowthlimit _secondarygrowthtimer _producequanitymin _producequanitymax _mainmesh _producemesh _seasonsofgrowth _everbearing_ _everbearingcycle _witherlimit _withertimer _currentgrowth _dead_ _location _unharvested _producetodrop) (break `/Game/Dynamic/CustomBPS/PlantSystem/F_Plants` (`self.PlantStruct`)))
  ;[1 1 1] Plant Code
  (if _unharvested
    (`|SpawnActorFromClass` "/Game/Dynamic/InventorySystem/Items/1ItemParent1.1ItemParent1_C" (`KismetMathLibrary.MakeTransform` (+ (`self.K2_GetActorLocation`) (0.0 0.0 100.0))) "AlwaysSpawn" "MultiplyWithRoot" null (`KismetMathLibrary.RandomIntegerInRange` _producequanitymin _producequanitymax) _producetodrop null)
    (if _everbearing_
      (setmembers `/Game/Dynamic/CustomBPS/PlantSystem/F_Plants` :`StructRef` (`self.PlantStruct`) :`Unharvested` false)
      (else
        (`self.K2_DestroyActor`)))))

(fn `LookAt`
  (returns (Message :type Text))
  (bind (_name _growthlimit _secondarygrowthlimit _secondarygrowthtimer _producequanitymin _producequanitymax _mainmesh _producemesh _seasonsofgrowth _everbearing_ _everbearingcycle _witherlimit _withertimer _currentgrowth _dead_ _location _unharvested) (break `/Game/Dynamic/CustomBPS/PlantSystem/F_Plants` (`self.PlantStruct`)))
  (bind _returnvalue (select `bool` _dead_ :`false` (`|FormatText` "Plant: {Name} Not Ready For Harvest" _name) :`true` (`|FormatText` "Plant: {Name} Dead" _name)))
  (if _dead_
    (return _returnvalue)
    (else
      (return (select `bool` _unharvested :`false` _returnvalue :`true` (`|FormatText` "Plant: {Name} Ready For Harvest" _name))))))

(fn `UserConstructionScript`)