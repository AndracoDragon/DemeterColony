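; Tilled-soil plot for the plant system, previewed as a green or red hologram by overlap until placed.
; Placing clears small plants through a harvest-interface box trace and applies a dynamic dirt material with collision.
; Seeding spawns a linked BP_Plant at the seed socket, destroyed with the plot.
; Watering darkens the dirt; an hourly Ultra Dynamic Sky callback handles weather-driven watering and dries it at hour 3.
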(event `self.ReceiveBeginPlay`
  (bind _dirt (`self.Dirt`))
  (if (`.placed_1_F38533294C427F706D8A1FAD679E2B53` (break `/Game/Dynamic/CustomBPS/PlantSystem/F_TillStruct` (`self.TillStruct`)))
    (`self.SetPlaceSaved`)
    (else
      (set `self.OriginalMat` (`PrimitiveComponent.GetMaterial` _dirt 0))
      (`PrimitiveComponent.SetMaterial` _dirt 0 "/Game/Static/Materials/CustomMats/MI_HologramGreen.MI_HologramGreen")
      (`PrimitiveComponent.SetCollisionEnabled` (`self.Dirt`) "NoCollision")))
  (bind _returnvalue (`GameplayStatics.GetActorOfClass` "/Game/Dynamic/UltraDynamicSky/Blueprints/Ultra_Dynamic_Sky.Ultra_Dynamic_Sky_C"))
  (bind _returnvalue_2 (`GameplayStatics.GetActorOfClass` "/Game/Dynamic/UltraDynamicSky/Blueprints/Ultra_Dynamic_Weather.Ultra_Dynamic_Weather_C"))
  (set `self.UDW` _returnvalue_2)
  (bind _output_get (set `self.UDS` _returnvalue))
  (add `/Game/Dynamic/UltraDynamicSky/Blueprints/Ultra_Dynamic_Sky.Hourly` _output_get (delegate `Dailies`)))

(event `DailyChecks`
  (bind _dynamicmat (`self.DynamicMat`))
  (set `self.Watered?` false)
  (`MaterialInstanceDynamic.SetScalarParameterValue` _dynamicmat "RoughAdjust" 1.0)
  (`MaterialInstanceDynamic.SetScalarParameterValue` _dynamicmat "Brightness" 1.0))

(event `Dailies`
  (params (Hour :type Integer))
  (if (== Hour 3)
    (`self.DailyChecks`)
    (else
      (switch `/Game/Dynamic/UltraDynamicSky/Blueprints/Enum/UDS_Weather_Display_Names` (`/Game/Dynamic/UltraDynamicSky/Blueprints/Ultra_Dynamic_Weather.ED_CurrentWeather` (`self.UDW`))
        (:`NewEnumerator0`
          _)
        (:`NewEnumerator1`
          _)
        (:`NewEnumerator2`
          _)
        (:`NewEnumerator3`
          _))
      (`/Game/Dynamic/CustomBPS/Interfaces/BPI_Watering.Water`))))

(event `self.CollisionBox.OnComponentBeginOverlap`
  (params (OverlappedComponent :type "PrimitiveComponent Object Reference") (OtherActor :type "Actor Object Reference") (OtherComp :type "PrimitiveComponent Object Reference") (OtherBodyIndex :type Integer) (bFromSweep :type Boolean) (SweepResult :type "HitResult Structure (by ref)"))
  (`self.IsBlocked`))

(event `IsBlocked`
  (if (or (not (`self.Set Place`)) (not (`.placed_1_F38533294C427F706D8A1FAD679E2B53` (break `/Game/Dynamic/CustomBPS/PlantSystem/F_TillStruct` (`self.TillStruct`)))))
    (`PrimitiveComponent.SetMaterial` (`self.Dirt`) 0 "/Game/Static/Materials/CustomMats/MI_HologramRed.MI_HologramRed")
    (set `self.Blocked` true)))

(event `self.CollisionBox.OnComponentEndOverlap`
  (params (OverlappedComponent :type "PrimitiveComponent Object Reference") (OtherActor :type "Actor Object Reference") (OtherComp :type "PrimitiveComponent Object Reference") (OtherBodyIndex :type Integer))
  (`self.IsUnblocked`))

(event `ClearSmallPlants`
  (params (CustomPC :type "/Game/Dynamic/CustomBPS/CustomPlayerController Object Reference"))
  (bind _returnvalue (`self.K2_GetActorLocation`))
  (bind _outhits (`KismetSystemLibrary.BoxTraceMulti` _returnvalue _returnvalue (44.0 44.0 20.0) (struct) "TraceTypeQuery5"))
  (for _array_element _outhits
    (bind (_bblockinghit _binitialoverlap _time _distance _location _impactpoint _normal _impactnormal _physmat _hitactor _hitcomponent) (`GameplayStatics.BreakHitResult` _array_element))
    (if (`KismetSystemLibrary.DoesImplementInterface` _hitcomponent "/Game/Dynamic/CustomBPS/Interfaces/BPI_Harvest.BPI_Harvest_C")
      (message `/Game/Dynamic/CustomBPS/Interfaces/BPI_Harvest.HitGrassBuild/Hoe` _hitcomponent _array_element))))

(event `IsUnblocked`
  (if (or (not (`self.Set Place`)) (not (`.placed_1_F38533294C427F706D8A1FAD679E2B53` (break `/Game/Dynamic/CustomBPS/PlantSystem/F_TillStruct` (`self.TillStruct`)))))
    (`PrimitiveComponent.SetMaterial` (`self.Dirt`) 0 "/Game/Static/Materials/CustomMats/MI_HologramGreen.MI_HologramGreen")
    (set `self.Blocked` false)))

(event `SetPlaceSaved`
  (bind _originalmat (`self.OriginalMat`))
  (`self.ClearSmallPlants` (stale `SetPlace` CustomPC) :!label _label)
  (set `self.Set Place` true)
  (`PrimitiveComponent.SetMaterial` (`self.Dirt`) 0 _originalmat)
  (bind _returnvalue (`KismetMaterialLibrary.CreateDynamicMaterialInstance` _originalmat))
  (set `self.DynamicMat` _returnvalue)
  (`PrimitiveComponent.SetMaterial` (`self.Dirt`) 0 _returnvalue)
  (`PrimitiveComponent.SetCollisionEnabled` (`self.Dirt`) "QueryAndPhysics"))

(event `SetPlace`
  (params (CustomPC :type "/Game/Dynamic/CustomBPS/CustomPlayerController Object Reference"))
  (if (not (`self.Blocked`))
    (`PrimitiveComponent.SetCollisionEnabled` (`self.CollisionBox`) "NoCollision")
    (goto _label)))

(event `/Game/Dynamic/CustomBPS/Interfaces/BPI_Watering.Seeded`
  (params (SeedToUse :type "/Game/Dynamic/InventorySystem/F_SlotStruct Structure"))
  (bind _tillstruct (`self.TillStruct`))
  (if (not (`.Seeded_6_33719F544D5BB48A8BC6978338847583` (break `/Game/Dynamic/CustomBPS/PlantSystem/F_TillStruct` _tillstruct)))
    (setmembers `/Game/Dynamic/CustomBPS/PlantSystem/F_TillStruct` :`StructRef` _tillstruct :`Seeded` true)
    (bind _returnvalue (`|SpawnActorFromClass` "/Game/Dynamic/CustomBPS/PlantSystem/BP_Plant.BP_Plant_C" (`KismetMathLibrary.MakeTransform` (`SceneComponent.GetSocketLocation` (`self.Dirt`) "SeedPileSocket")) "Undefined" "MultiplyWithRoot" null SeedToUse self null))
    (set `self.Plant` _returnvalue)))

(event `/Game/Dynamic/CustomBPS/Interfaces/BPI_Watering.DestroyHoeEarth`
  (bind _plant (`self.Plant`)
    (:`then`
      (`self.K2_DestroyActor` _plant))
    (:`else`
      _))
  (`self.K2_DestroyActor` self))

(event `/Game/Dynamic/CustomBPS/Interfaces/BPI_Watering.Water`
  (bind _dynamicmat (`self.DynamicMat`))
  (set `self.Watered?` true)
  (`MaterialInstanceDynamic.SetScalarParameterValue` _dynamicmat "RoughAdjust" 0.0)
  (`MaterialInstanceDynamic.SetScalarParameterValue` _dynamicmat "Brightness" 0.5))

(fn `UserConstructionScript`)