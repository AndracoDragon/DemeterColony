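; Sliding inner door for the Town Center that opens when an actor implementing BPI_Door enters its Box trigger.
; The OpenDoor timeline lerps the StaticMesh from its starting relative location to a fixed offset.
; On exit, Close rescans the Box and reverses the timeline if no BPI_Door actor remains.
; StayOpen only clears inside that scan loop, so an empty overlap list leaves the door open.
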(event `self.ReceiveBeginPlay`
  (set `self.Relative Location` (`SceneComponent.RelativeLocation` (`self.StaticMesh`))))

(event `Open`
  (if (not (`self.StayOpen?`))
    (set `self.StayOpen?` true)
    (bind (_direction _newtrack_0) (`Timeline|OpenDoor` :!label _label)
      (:`Update`
        (`SceneComponent.K2_SetRelativeLocation` (`self.StaticMesh`) (`KismetMathLibrary.VLerp` (`self.Relative Location`) (0.0 175.0 0.0) _newtrack_0) false false)))))

(event `Close`
  (for _array_element (`PrimitiveComponent.GetOverlappingActors` (`self.Box`) "/Script/Engine.Actor")
    (if (`KismetSystemLibrary.DoesImplementInterface` _array_element "/Game/Dynamic/CustomBPS/Interfaces/BPI_Door.BPI_Door_C")
      (set `self.StayOpen?` true)
      (break)
      (else
        (set `self.StayOpen?` false))))
  (if (not (`self.StayOpen?`))
    (goto _label :!via `Reverse`)))

(event `self.Box.OnComponentBeginOverlap`
  (params (OverlappedComponent :type "PrimitiveComponent Object Reference") (OtherActor :type "Actor Object Reference") (OtherComp :type "PrimitiveComponent Object Reference") (OtherBodyIndex :type Integer) (bFromSweep :type Boolean) (SweepResult :type "HitResult Structure (by ref)"))
  (if (`KismetSystemLibrary.DoesImplementInterface` OtherActor "/Game/Dynamic/CustomBPS/Interfaces/BPI_Door.BPI_Door_C")
    (`self.Open`)))

(event `self.Box.OnComponentEndOverlap`
  (params (OverlappedComponent :type "PrimitiveComponent Object Reference") (OtherActor :type "Actor Object Reference") (OtherComp :type "PrimitiveComponent Object Reference") (OtherBodyIndex :type Integer))
  (if (`KismetSystemLibrary.DoesImplementInterface` OtherActor "/Game/Dynamic/CustomBPS/Interfaces/BPI_Door.BPI_Door_C")
    (`self.Close`)))

(fn `UserConstructionScript`)