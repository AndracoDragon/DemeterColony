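; Instanced foliage Blueprint that removes grass instances when hit and regrows them from small seedlings.
; HitGrass stores the hit instance's location and rotation at reduced scale, conditionally removes it, then calls Regrow.
; Regrow sphere-traces each stored spot and adds a small instance where nothing blocks it.
; GrowItems scales these toward full size by removing and re-adding them slightly larger, re-calling itself after a short Delay.
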(event `/Game/Dynamic/CustomBPS/Interfaces/BPI_Harvest.HitGrass`
  (params (CustomPC :type "/Game/Dynamic/CustomBPS/CustomPlayerController Object Reference") (`Hit Result` :type "HitResult Structure"))
  (bind (_bblockinghit _binitialoverlap _time _distance _location _impactpoint _normal _impactnormal _physmat _hitactor _hitcomponent _hitbonename _bonename _hititem) (`GameplayStatics.BreakHitResult` `Hit Result`))
  (bind _transform (`self.Transform`))
  (bind _returnvalue (`KismetMathLibrary.MakeTransform` (.location (`self.GetInstanceTransform` _hititem true)) (.rotation (`self.GetInstanceTransform` _hititem true)) (0.1 0.1 0.1)))
  ;[1 1 1] Gets the instance being hit.
  ;[1 1 1] Checks to see if i already have this transform in the regrwth array
  (if (`KismetArrayLibrary.Array_IsValidIndex` _transform)
    (for _array_element _transform
      (if (== (.location _array_element) (.location _returnvalue))
        (set `self.Condition` false)
        (else
          (`KismetArrayLibrary.Array_Add` _transform _returnvalue)
          (set `self.Condition` true))))
    (else
      (`KismetArrayLibrary.Array_Add` _transform _returnvalue)))
  (if (not (`self.Condition`))
    ;[1 1 1] Removes and Starts regrowth
    (`self.RemoveInstance` _hititem)
    (`self.Regrow`)))

(event `Regrow`
  ;[1 1 1] Tells things to regrow
  (`/Engine/EditorBlueprintResources/StandardMacros.DoOnce` false :!label _label
    (:`Completed`
      (for _array_element (`self.Transform`)
        (bind _returnvalue (+ (.location _array_element) (0.0 0.0 20.0)))
        (bind (_outhit _returnvalue_2) (`KismetSystemLibrary.SphereTraceSingle` :`Start` _returnvalue :`End` _returnvalue :`Radius` 30.0 :`TraceChannel` "TraceTypeQuery4" :`DrawDebugType` "ForDuration"))
        (if (not _returnvalue_2)
          (bind _returnvalue_3 (`self.AddInstance` _array_element true))
          (`KismetArrayLibrary.Array_Add` (`self.Hit Item`) _returnvalue_3)
          (`KismetSystemLibrary.Delay` 0.2)
          (`self.Grow Items`)))
      (goto _label :!via `Reset`))))

(event `Grow Items`
  (bind _hit_item (`self.Hit Item`))
  ;[1 1 1] Grows things in increments
  (for (_array_element _array_index) (`self.Hit Item`)
    (`KismetArrayLibrary.Array_Remove` _hit_item _array_index)
    (bind _outinstancetransform (`self.GetInstanceTransform` _array_element true))
    (if (not (== (.scale _outinstancetransform) (1.0 1.0 1.0) :`ErrorTolerance` 0.1))
      (`self.RemoveInstance` _array_element)
      (bind _returnvalue (`self.AddInstance` (`KismetMathLibrary.MakeTransform` (.location _outinstancetransform) (.rotation _outinstancetransform) (+ (.scale _outinstancetransform) (0.01 0.01 0.01))) true))
      (`KismetArrayLibrary.Array_Add` _hit_item _returnvalue)
      (bind _result (`/Engine/EditorBlueprintResources/StandardMacros.IncrementInt` (`self.Iterations`))
        (:`  `
          (`KismetSystemLibrary.Delay` 0.2)
          (`self.Grow Items`))))))