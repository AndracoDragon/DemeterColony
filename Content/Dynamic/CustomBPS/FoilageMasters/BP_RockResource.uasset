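; Instanced-mesh rock resource that players mine with a pickaxe for loot and that can regrow over time.
; HitRock damages the hit instance's tracked health by tool level, warning on disallowed tiers; level 0 skips straight to removal.
; Removed instances are recorded in DestroyedInstances and roll loot-table pickups.
; An Ultra Dynamic Sky hourly event triggers Regrow at hour 2, re-adding instances by chance where a sphere trace finds no obstruction.
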(event `self.ReceiveBeginPlay`
  (bind _returnvalue (`GameplayStatics.GetActorOfClass` "/Game/Dynamic/UltraDynamicSky/Blueprints/Ultra_Dynamic_Sky.Ultra_Dynamic_Sky_C"))
  (bind _output_get (set `self.UDS` _returnvalue))
  (bind _returnvalue_2 (`GameplayStatics.GetActorOfClass` "/Game/Dynamic/UltraDynamicSky/Blueprints/Ultra_Dynamic_Weather.Ultra_Dynamic_Weather_C"))
  (set `self.UDW` _returnvalue_2)
  (add `/Game/Dynamic/UltraDynamicSky/Blueprints/Ultra_Dynamic_Sky.Hourly` _output_get (delegate `CheckSeason`))
  (for _index (range (+ (`self.GetInstanceCount`) 1))
    (`KismetArrayLibrary.Array_Set` (`self.Instances`) _index (make `/Game/Dynamic/CustomBPS/FoilageMasters/F_FoilageStruct` (`self.Health`)) true)))

(event `CheckSeason`
  (params (Hour :type Integer))
  (if (== Hour 2)
    (`self.Regrow`)))

(event `/Game/Dynamic/CustomBPS/Interfaces/BPI_Harvest.HitRock`
  (params (CustomPC :type "/Game/Dynamic/CustomBPS/CustomPlayerController Object Reference") (`Hit Result` :type "HitResult Structure"))
  (bind (_bblockinghit _binitialoverlap _time _distance _location _impactpoint _normal _impactnormal _physmat _hitactor _hitcomponent _hitbonename _bonename _hititem) (`GameplayStatics.BreakHitResult` `Hit Result`))
  (bind _loottable (`self.LootTable`))
  (bind _itemspawn__location (`KismetMathLibrary.BreakTransform` (`self.ItemSpawn?`)))
  (bind _instances (`self.Instances`))
  (bind _destroyedinstances (`self.DestroyedInstances`))
  (bind _output (`|GetArrayItem` _instances _hititem))
  (bind _level (`/Game/Dynamic/CustomBPS/ToolSystem/BP_Tool.Level` (`/Game/Dynamic/CustomBPS/CustomPlayerController.ToolVar` CustomPC)))
  (bind _output_dthandle (break `/Game/Dynamic/InventorySystem/F_SlotStruct` (`|GetArrayItem` _loottable (`KismetMathLibrary.RandomIntegerInRange` 0 (`KismetArrayLibrary.Array_Length` _loottable)))))
  (bind _returnvalue (- (`.Health_2_8243E3F24CEF7CF1EBDD0C929541D226` (break `/Game/Dynamic/CustomBPS/FoilageMasters/F_FoilageStruct` _output)) (`self.DamageToDo`)))
  ;[1 1 1] Gets the instance being hit.
  (switch `/Game/Dynamic/InventorySystem/Enum_NonConsumableType` (`/Game/Dynamic/CustomBPS/ToolSystem/BP_Tool.Tool` (`/Game/Dynamic/CustomBPS/CustomPlayerController.ToolVar` CustomPC))
    (:`NewEnumerator2`
      (set `self.ItemSpawn?` (`self.GetInstanceTransform` _hititem true))
      ;[1 1 1] HandlesDamage
      (switch `int` (`/Game/Dynamic/CustomBPS/ToolSystem/BP_Tool.Level` (`/Game/Dynamic/CustomBPS/CustomPlayerController.ToolVar` CustomPC))
        (:`0`
          ;[1 1 1] Checks to see if it is already added to array
          (bind _keys (`BlueprintMapLibrary.Map_Keys` _destroyedinstances :!label _label))
          (if (== (`KismetArrayLibrary.Array_Find` _keys _hititem) -1)
            (`BlueprintMapLibrary.Map_Add` _destroyedinstances _hititem))
          ;[1 1 1] Removes, loots, and Starts regrowth
          (`self.RemoveInstance` _hititem)
          (if (`KismetArrayLibrary.Array_IsValidIndex` (`self.LootTable`))
            (for _ (range (+ (* _level 2) 1))
              (if (<= (`KismetMathLibrary.RandomIntegerInRange` 1 100) (`self.LootChance`))
                (`|SpawnActorFromClass` "/Game/Dynamic/InventorySystem/Items/1ItemParent1.1ItemParent1_C" (`KismetMathLibrary.MakeTransform` (+ _itemspawn__location (0.0 0.0 100.0))) "AdjustIfPossibleButAlwaysSpawn" "MultiplyWithRoot" null (* _level (`KismetMathLibrary.RandomIntegerInRange` (`self.MinQuanity`) (`self.MaxQuanity`))) _output_dthandle null)))))
        (:`1`
          (if (`self.Level1`)
            (set `self.DamageToDo` 15)
            (bind _structout (setmembers `/Game/Dynamic/CustomBPS/FoilageMasters/F_FoilageStruct` :`StructRef` _output :`Health` _returnvalue :!label _label_2))
            (`KismetArrayLibrary.Array_Set` _instances _hititem _structout)
            (if (<= _returnvalue 0)
              (goto _label))
            (else
              (`/Game/Dynamic/Widgets/HUD/PlayerHUD_W.WeakTool` (`/Game/Dynamic/Widgets/PlayerMenu/PlayerMenuBase_W.PlayerHUD_W` (`/Game/Dynamic/ThirdPerson/Blueprints/BP_ThirdPersonCharacter.PlayerHud` (`/Game/Dynamic/CustomBPS/CustomPlayerController.As BP Third Person Character` CustomPC))) :!label _label_3))))
        (:`2`
          (if (`self.Level2`)
            (set `self.DamageToDo` 35)
            (goto _label_2)
            (else
              (goto _label_3))))
        (:`3`
          (if (`self.Level3`)
            (set `self.DamageToDo` 50)
            (goto _label_2)
            (else
              (goto _label_3))))))))

(event `Regrow`
  (bind _destroyedinstances (`self.DestroyedInstances`))
  ;[1 1 1] Tells things to regrow
  (`/Engine/EditorBlueprintResources/StandardMacros.DoOnce` false :!label _label_4
    (:`Completed`
      (bind _keys (`BlueprintMapLibrary.Map_Keys` (`self.DestroyedInstances`)))
      (if (`KismetArrayLibrary.Array_IsValidIndex` _keys)
        (for (_ _array_index) _keys
          (bind _keys_2 (`BlueprintMapLibrary.Map_Keys` _destroyedinstances))
          (bind _values (`BlueprintMapLibrary.Map_Values` _destroyedinstances))
          (if (<= (`KismetMathLibrary.RandomIntegerInRange` 1 100) (`self.ChancetoSpawn`))
            (bind _output (`|GetArrayItem` _values (`|GetArrayItem` _keys_2 _array_index)))
            (bind _returnvalue (+ (.location _output) (0.0 0.0 20.0)))
            (bind (_outhit _returnvalue_2) (`KismetSystemLibrary.SphereTraceSingle` :`Start` _returnvalue :`End` _returnvalue :`Radius` 30.0 :`TraceChannel` "TraceTypeQuery1" :`DrawDebugType` "ForDuration"))
            (if (not _returnvalue_2)
              (`self.AddInstance` (`KismetMathLibrary.MakeTransform` (.location _output)) true)
              (`BlueprintMapLibrary.Map_Remove` (`self.DestroyedInstances`) _array_index))))
        (goto _label_4 :!via `Reset`)))))