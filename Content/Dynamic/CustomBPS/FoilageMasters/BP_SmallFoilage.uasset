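; Small foliage instanced-mesh master that players clear with tools and that regrows over time.
; Hoe, hammer or shovel hits remove the instance and store its transform, with the shovel also spawning loot scaled by tool level.
; An Ultra Dynamic Sky hourly check randomly re-adds unobstructed instances at small scale, then GrowItems enlarges them by re-creating them.
; Ultra Dynamic Weather's season controls whether the foliage is hidden.
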(event `self.ReceiveBeginPlay`
  (bind _returnvalue (`GameplayStatics.GetActorOfClass` "/Game/Dynamic/UltraDynamicSky/Blueprints/Ultra_Dynamic_Sky.Ultra_Dynamic_Sky_C"))
  (bind _output_get (set `self.UDS` _returnvalue))
  (bind _returnvalue_2 (`GameplayStatics.GetActorOfClass` "/Game/Dynamic/UltraDynamicSky/Blueprints/Ultra_Dynamic_Weather.Ultra_Dynamic_Weather_C"))
  (bind _output_get_2 (set `self.UDW` _returnvalue_2))
  (add `/Game/Dynamic/UltraDynamicSky/Blueprints/Ultra_Dynamic_Sky.Hourly` _output_get (delegate `CheckSeason`))
  (bind _ascustom_player_controller (cast `/Game/Dynamic/CustomBPS/CustomPlayerController` (`GameplayStatics.GetPlayerController` 0)))
  (set `self.As Custom Player Controller` _ascustom_player_controller)
  (if (== (`KismetMathLibrary.FFloor` (`/Game/Dynamic/UltraDynamicSky/Blueprints/Ultra_Dynamic_Weather.Season` _output_get_2)) 4) :!label _label
    (`self.SetHiddenInGame` true)
    (else
      (`self.SetHiddenInGame` false))))

(event `CheckSeason`
  (params (Hour :type Integer))
  (if (== Hour 2)
    (`KismetSystemLibrary.Delay` 1.0)
    (`self.Regrow`)
    (goto _label)))

(event `Hit Event`
  (params (HitResult :type "HitResult Structure"))
  (bind (_bblockinghit _binitialoverlap _time _distance _location _impactpoint _normal _impactnormal _physmat _hitactor _hitcomponent _hitbonename _bonename _hititem) (`GameplayStatics.BreakHitResult` HitResult))
  (bind (_bblockinghit_2 _binitialoverlap_2 _time_2 _distance_2 _location_2 _impactpoint_2 _normal_2 _impactnormal_2 _physmat_2 _hitactor_2 _hitcomponent_2 _hitbonename_2 _bonename_2 _hititem_2) (`GameplayStatics.BreakHitResult` HitResult))
  (bind _transform (`self.Transform`))
  (bind _loottable (`self.LootTable`))
  (bind _itemspawn__location (`KismetMathLibrary.BreakTransform` (`self.ItemSpawn?`)))
  (bind _transform_2 (`self.Transform`))
  (bind _outinstancetransform (`self.GetInstanceTransform` _hititem true))
  (bind _outinstancetransform_2 (`self.GetInstanceTransform` _hititem_2 true))
  (bind _level (`/Game/Dynamic/CustomBPS/ToolSystem/BP_Tool.Level` (`/Game/Dynamic/CustomBPS/CustomPlayerController.ToolVar` (`self.As Custom Player Controller`))))
  (bind _output_dthandle (break `/Game/Dynamic/InventorySystem/F_SlotStruct` (`|GetArrayItem` _loottable (`KismetMathLibrary.RandomIntegerInRange` 0 (`KismetArrayLibrary.Array_Length` _loottable)))))
  ;[1 1 1] Gets the instance being hit.
  (switch `/Game/Dynamic/InventorySystem/Enum_NonConsumableType` (`/Game/Dynamic/CustomBPS/ToolSystem/BP_Tool.Tool` (`/Game/Dynamic/CustomBPS/CustomPlayerController.ToolVar` (`self.As Custom Player Controller`)))
    (:`NewEnumerator0`
      ;[0.2 0 1] HammerFoilageRemove
      (set `self.ItemSpawn?` _outinstancetransform :!label _label_2)
      (if (== (`KismetArrayLibrary.Array_Find` _transform_2 (`KismetMathLibrary.MakeTransform` (.location _outinstancetransform) (.rotation _outinstancetransform) (0.1 0.1 0.1))) -1)
        (`KismetArrayLibrary.Array_Add` _transform_2))
      (`self.RemoveInstance` _hititem))
    (:`NewEnumerator1`
      (set `self.ItemSpawn?` _outinstancetransform_2)
      ;[1 1 1] Checks to see if it is already added to array
      (if (== (`KismetArrayLibrary.Array_Find` _transform (`KismetMathLibrary.MakeTransform` (.location _outinstancetransform_2) (.rotation _outinstancetransform_2) (0.1 0.1 0.1))) -1) :!label _label_3
        (`KismetArrayLibrary.Array_Add` _transform))
      ;[1 1 1] Removes, loots, and Starts regrowth
      (`self.RemoveInstance` _hititem_2)
      (if (`KismetArrayLibrary.Array_IsValidIndex` (`self.LootTable`))
        (for _ (range (+ (* _level 2) 1))
          (if true
            (`|SpawnActorFromClass` "/Game/Dynamic/InventorySystem/Items/1ItemParent1.1ItemParent1_C" (`KismetMathLibrary.MakeTransform` (+ _itemspawn__location (0.0 0.0 100.0))) "AdjustIfPossibleButAlwaysSpawn" "MultiplyWithRoot" null (* _level (`KismetMathLibrary.RandomIntegerInRange` 1 3)) _output_dthandle null)))))
    (:`NewEnumerator5`
      (goto _label_2))))

(event `Industrial`
  ;[1 1 1] Checks to see if it is already added to array
  (goto _label_3))

(event `Regrow`
  (bind _transform (`self.Transform`))
  ;[1 1 1] Tells things to regrow
  (`/Engine/EditorBlueprintResources/StandardMacros.DoOnce` false :!label _label_4
    (:`Completed`
      (if (`KismetArrayLibrary.Array_IsValidIndex` _transform)
        (for _array_element _transform
          (if (<= (`KismetMathLibrary.RandomIntegerInRange` 1 100) 33)
            (bind _returnvalue (+ (.location _array_element) (0.0 0.0 20.0)))
            (bind (_outhit _returnvalue_2) (`KismetSystemLibrary.SphereTraceSingle` :`Start` _returnvalue :`End` _returnvalue :`Radius` 30.0 :`TraceChannel` "TraceTypeQuery1" :`DrawDebugType` "ForDuration"))
            (if (not _returnvalue_2)
              (bind _returnvalue_3 (`self.AddInstance` (`KismetMathLibrary.MakeTransform` (.location _array_element) (struct) (0.1 0.1 0.1)) true))
              (`KismetArrayLibrary.Array_Remove` _transform (`KismetArrayLibrary.Array_Find` _transform _array_element))
              (`KismetArrayLibrary.Array_Add` (`self.Hit Item`) _returnvalue_3)
              (`KismetSystemLibrary.Delay` 0.2)
              (`self.Grow Items`))))
        (goto _label_4 :!via `Reset`)))))

(event `Grow Items`
  (bind _hit_item (`self.Hit Item`))
  ;[1 1 1] Grows things in increments
  (for (_array_element _array_index) (`self.Hit Item`)
    (`KismetArrayLibrary.Array_Remove` _hit_item _array_index)
    (bind _outinstancetransform (`self.GetInstanceTransform` _array_element true))
    (if (not (== (.scale _outinstancetransform) (1.0 1.0 1.0) :`ErrorTolerance` 0.1))
      (`self.RemoveInstance` _array_element)
      (bind _returnvalue (`self.AddInstance` (`KismetMathLibrary.MakeTransform` (.location _outinstancetransform) (.rotation _outinstancetransform) (+ (.scale _outinstancetransform) (0.1 0.1 0.1))) true))
      (`KismetArrayLibrary.Array_Add` _hit_item _returnvalue)
      (bind _result (`/Engine/EditorBlueprintResources/StandardMacros.IncrementInt` (`self.Iterations`))
        (:`  `
          (`KismetSystemLibrary.PrintString` (`KismetStringLibrary.Conv_IntToString` _result))
          (`KismetSystemLibrary.Delay` 0.2))))))