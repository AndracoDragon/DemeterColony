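; BP_Depression is a precipitation actor that keeps a Niagara effect hovering above the player character.
; On BeginPlay it caches the player as BP_ThirdPersonCharacter, then assigns the configured Niagara asset to its component.
; A looping short-interval timer, used in place of Tick, moves the actor to the player's location with a fixed upward offset.
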(event `self.ReceiveBeginPlay`
  (bind _asbp_third_person_character (cast `/Game/Dynamic/ThirdPerson/Blueprints/BP_ThirdPersonCharacter` (`GameplayStatics.GetPlayerCharacter` 0)))
  (set `self.As BP Third Person Character` _asbp_third_person_character)
  (`self.Percipatate`))

(event `Percipatate`
  (`NiagaraComponent.SetAsset` (`self.Niagara`) (`self.NiagaraAsset`) true)
  (bind _returnvalue (`KismetSystemLibrary.K2_SetTimerDelegate` (delegate `Follow PLayer`) 0.01 true))
  (set `self.PercipatateTimer` _returnvalue))

(event `Follow PLayer`
  (`self.K2_SetActorLocation` (`KismetMathLibrary.MakeVector` (.x (`self.K2_GetActorLocation` (`self.As BP Third Person Character`))) (.y (`self.K2_GetActorLocation` (`self.As BP Third Person Character`))) (+ (.z (`self.K2_GetActorLocation` (`self.As BP Third Person Character`))) 300.0))))

(fn `UserConstructionScript`)