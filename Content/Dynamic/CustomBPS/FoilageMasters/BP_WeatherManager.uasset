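; Weather manager that ties Ultra Dynamic Sky's clock to Ultra Dynamic Weather and seasonal foliage tinting.
; An hourly callback prints the date and, at hour 2, picks a new random weather type and checks the season.
; Months 1–4 map directly to Spring through Winter, setting the weather season and pushing that season's color into the MPC_1Foilage parameter collection.
; A separate CloudSettings function writes sun and cloud values to a SkyBox.
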(event `self.ReceiveBeginPlay`
  (add `/Game/Dynamic/UltraDynamicSky/Blueprints/Ultra_Dynamic_Sky.Hourly` (`self.IltradynamicSky`) (delegate `Test`)))

(event `Change Weather`
  (`/Game/Dynamic/UltraDynamicSky/Blueprints/Weather_Effects/System/Random_Weather_Variation.Select New Random Weather Type` (`/Game/Dynamic/UltraDynamicSky/Blueprints/Ultra_Dynamic_Weather.Random_Weather_Variation` (`self.UltraDynamicWeather`)) true)
  (`self.Check Season`))

(event `Test`
  (params (Hour :type Integer))
  (`|ExecutionSequence`
    (:`then_0`
      (if (== Hour 2)
        (`self.Change Weather`)))
    (:`then_1`
      (bind _current_date_and_time (`/Game/Dynamic/UltraDynamicSky/Blueprints/Ultra_Dynamic_Sky.Get Current Date and Time` (`self.IltradynamicSky`)))
      (bind (_year _month _day) (`KismetMathLibrary.BreakDateTime` _current_date_and_time))
      (`KismetSystemLibrary.PrintString` (`KismetTextLibrary.Conv_TextToString` (`|FormatText` "Year: {year} Month: {month} Day: {Day}" _year _month _day))))))

(event `Check Season`
  (bind _ultradynamicweather (`self.UltraDynamicWeather`))
  (bind _month (`/Game/Dynamic/UltraDynamicSky/Blueprints/Ultra_Dynamic_Sky.Month` (`self.IltradynamicSky`)))
  (bind _returnvalue (`KismetMathLibrary.Conv_IntToDouble` _month))
  (switch `int` _month
    (:`1`
      (set `/Game/Dynamic/UltraDynamicSky/Blueprints/Ultra_Dynamic_Weather.Season` _returnvalue _ultradynamicweather)
      (`/Game/Dynamic/UltraDynamicSky/Blueprints/Weather_Effects/System/Ultra_Dynamic_Weather_Interface.Set Season` _ultradynamicweather)
      (set `self.SeasonColor` "NewEnumerator0"))
    (:`2`
      (set `/Game/Dynamic/UltraDynamicSky/Blueprints/Ultra_Dynamic_Weather.Season` _returnvalue _ultradynamicweather)
      (`/Game/Dynamic/UltraDynamicSky/Blueprints/Weather_Effects/System/Ultra_Dynamic_Weather_Interface.Set Season` _ultradynamicweather)
      (set `self.SeasonColor` "NewEnumerator1"))
    (:`3`
      (set `/Game/Dynamic/UltraDynamicSky/Blueprints/Ultra_Dynamic_Weather.Season` _returnvalue _ultradynamicweather)
      (`/Game/Dynamic/UltraDynamicSky/Blueprints/Weather_Effects/System/Ultra_Dynamic_Weather_Interface.Set Season` _ultradynamicweather)
      (set `self.SeasonColor` "NewEnumerator2"))
    (:`4`
      (set `/Game/Dynamic/UltraDynamicSky/Blueprints/Ultra_Dynamic_Weather.Season` _returnvalue _ultradynamicweather)
      (`/Game/Dynamic/UltraDynamicSky/Blueprints/Weather_Effects/System/Ultra_Dynamic_Weather_Interface.Set Season` _ultradynamicweather)
      (set `self.SeasonColor` "NewEnumerator3")))
  (`self.Change Color`))

(event `Change Color`
  (bind _wintercolor (`self.WinterColor`))
  (bind _fallcolor (`self.FallColor`))
  (bind _springcolor (`self.SpringColor`))
  (bind _summercolor (`self.SummerColor`))
  (switch `/Game/Dynamic/CustomBPS/FoilageMasters/Enum_Seasons` (`self.SeasonColor`)
    (:`NewEnumerator0`
      (`KismetMaterialLibrary.SetVectorParameterValue` "/Game/Dynamic/CustomBPS/FoilageMasters/MPC_1Foilage.MPC_1Foilage" "Color/Brightness" _springcolor)
      (`KismetMaterialLibrary.SetVectorParameterValue` "/Game/Dynamic/CustomBPS/FoilageMasters/MPC_1Foilage.MPC_1Foilage" "Ground Tint" _springcolor))
    (:`NewEnumerator1`
      (`KismetMaterialLibrary.SetVectorParameterValue` "/Game/Dynamic/CustomBPS/FoilageMasters/MPC_1Foilage.MPC_1Foilage" "Color/Brightness" _summercolor)
      (`KismetMaterialLibrary.SetVectorParameterValue` "/Game/Dynamic/CustomBPS/FoilageMasters/MPC_1Foilage.MPC_1Foilage" "Ground Tint" _summercolor))
    (:`NewEnumerator2`
      (`KismetMaterialLibrary.SetVectorParameterValue` "/Game/Dynamic/CustomBPS/FoilageMasters/MPC_1Foilage.MPC_1Foilage" "Color/Brightness" _fallcolor)
      (`KismetMaterialLibrary.SetVectorParameterValue` "/Game/Dynamic/CustomBPS/FoilageMasters/MPC_1Foilage.MPC_1Foilage" "Ground Tint" _fallcolor))
    (:`NewEnumerator3`
      (`KismetMaterialLibrary.SetVectorParameterValue` "/Game/Dynamic/CustomBPS/FoilageMasters/MPC_1Foilage.MPC_1Foilage" "Color/Brightness" _wintercolor)
      (`KismetMaterialLibrary.SetVectorParameterValue` "/Game/Dynamic/CustomBPS/FoilageMasters/MPC_1Foilage.MPC_1Foilage" "Ground Tint" _wintercolor))))

(fn `CloudSettings`
  (params (`Sun brightness` :type "Float (double-precision)" :default 50.0) (`Cloud opacity` :type "Float (double-precision)" :default 1.0) (NoisePower1 :type "Float (single-precision)" :default 1.0) (NoisePower2 :type "Float (single-precision)" :default 2.0) (`Cloud color` :type "LinearColor Structure" :default (struct :`R` 0.854902 :`G` 0.917647 :`B` 1.0 :`A` 1.0)))
  (returns (NewParam :type Boolean))
  (bind _skybox (`self.SkyBox`))
  (set `/Engine/EngineSky/BP_Sky_Sphere.Sun brightness` `Sun brightness` _skybox)
  (set `/Engine/EngineSky/BP_Sky_Sphere.Cloud opacity` `Cloud opacity` _skybox)
  (set `/Engine/EngineSky/BP_Sky_Sphere.NoisePower1` NoisePower1 _skybox)
  (set `/Engine/EngineSky/BP_Sky_Sphere.NoisePower2` NoisePower2 _skybox)
  (set `/Engine/EngineSky/BP_Sky_Sphere.Cloud color` `Cloud color` _skybox)
  (return false))

(fn `UserConstructionScript`)