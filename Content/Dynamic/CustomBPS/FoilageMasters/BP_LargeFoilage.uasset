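; Instanced large-foliage Blueprint for choppable plants that drop loot and regrow.
; HitEvent checks the player's axe level, damaging per-instance health or showing a weak-tool warning; level 0 removes instantly.
; Removal saves the transform in a map and spawns LootTable items scaled by tool level.
; Ultra Dynamic Sky's hourly event triggers regrowth at hour 2: random, sphere-trace-clear spots get small instances, which GrowItems re-adds at increasing scale.
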(event `self.ReceiveBeginPlay`
  (bind _returnvalue (`GameplayStatics.GetActorOfClass` "/Game/Dynamic/UltraDynamicSky/Blueprints/Ultra_Dynamic_Sky.Ultra_Dynamic_Sky_C"))
  (bind _output_get (set `self.UDS` _returnvalue))
  (bind _returnvalue_2 (`GameplayStatics.GetActorOfClass` "/Game/Dynamic/UltraDynamicSky/Blueprints/Ultra_Dynamic_Weather.Ultra_Dynamic_Weather_C"))
  (set `self.UDW` _returnvalue_2)
  (add `/Game/Dynamic/UltraDynamicSky/Blueprints/Ultra_Dynamic_Sky.Hourly` _output_get (delegate `CheckSeason`))
  (bind _ascustom_player_controller (cast `/Game/Dynamic/CustomBPS/CustomPlayerController` (`GameplayStatics.GetPlayerController` 0)))
  (set `self.As Custom Player Controller` _ascustom_player_controller)
  (for _index (range (+ (`self.GetInstanceCount`) 1))
    (`KismetArrayLibrary.Array_Set` (`self.Instances`) _index (make `/Game/Dynamic/CustomBPS/FoilageMasters/F_FoilageStruct` (`self.Health`)) true)))

(event `CheckSeason`
  (params (Hour :type Integer))
  (if (== Hour 2)
    (`KismetSystemLibrary.Delay` 1.0)
    (`self.Regrow`)))

(event `Industrial`
  (bind _loottable (`self.LootTable`))
  (bind _itemspawn__location (`KismetMathLibrary.BreakTransform` (`self.ItemSpawn?`)))
  (bind _level (`/Game/Dynamic/CustomBPS/ToolSystem/BP_Tool.Level` (`/Game/Dynamic/CustomBPS/CustomPlayerController.ToolVar` (`self.As Custom Player Controller`))))
  (bind _output_dthandle (break `/Game/Dynamic/InventorySystem/F_SlotStruct` (`|GetArrayItem` _loottable (`KismetMathLibrary.RandomIntegerInRange` 0 (`KismetArrayLibrary.Array_Length` _loottable)))))
  ;[1 1 1] Checks to see if it is already added to array
  (bind (_bblockinghit _binitialoverlap _time _distance _location _impactpoint _normal _impactnormal _physmat _hitactor _hitcomponent _hitbonename _bonename _hititem) (`GameplayStatics.BreakHitResult` (stale `Hit Event` HitResult)))
  (`BlueprintMapLibrary.Map_Add` (`self.DestroyedInstances`) _hititem (`KismetMathLibrary.MakeTransform` (.location (`self.GetInstanceTransform` _hititem true)) (.rotation (`self.GetInstanceTransform` _hititem true)) (0.1 0.1 0.1)) :!label _label)
  ;[1 1 1] Removes, loots, and Starts regrowth
  (`self.RemoveInstance` _hititem :!label _label_2)
  (if (`KismetArrayLibrary.Array_IsValidIndex` (`self.LootTable`))
    (for _ (range (+ (* _level 2) 1))
      (if true
        (`|SpawnActorFromClass` "/Game/Dynamic/InventorySystem/Items/1ItemParent1.1ItemParent1_C" (`KismetMathLibrary.MakeTransform` (+ _itemspawn__location (0.0 0.0 100.0))) "AdjustIfPossibleButAlwaysSpawn" "MultiplyWithRoot" null (* _level (`KismetMathLibrary.RandomIntegerInRange` (`self.MinQuanity`) (`self.MaxQuanity`))) _output_dthandle null)))))

(event `Hit Event`
  (params (HitResult :type "HitResult Structure"))
  (bind (_bblockinghit _binitialoverlap _time _distance _location _impactpoint _normal _impactnormal _physmat _hitactor _hitcomponent _hitbonename _bonename _hititem) (`GameplayStatics.BreakHitResult` HitResult))
  (bind _instances (`self.Instances`))
  (bind _output (`|GetArrayItem` _instances _hititem))
  (bind _returnvalue (- (`.Health_2_8243E3F24CEF7CF1EBDD0C929541D226` (break `/Game/Dynamic/CustomBPS/FoilageMasters/F_FoilageStruct` _output)) (`self.DamageToDo`)))
  ;[1 1 1] Gets the instance being hit.
  (switch `/Game/Dynamic/InventorySystem/Enum_NonConsumableType` (`/Game/Dynamic/CustomBPS/ToolSystem/BP_Tool.Tool` (`/Game/Dynamic/CustomBPS/CustomPlayerController.ToolVar` (`self.As Custom Player Controller`)))
    (:`NewEnumerator9`
      (set `self.ItemSpawn?` (`self.GetInstanceTransform` _hititem true))
      ;[1 1 1] HandlesDamage
      (switch `int` (`/Game/Dynamic/CustomBPS/ToolSystem/BP_Tool.Level` (`/Game/Dynamic/CustomBPS/CustomPlayerController.ToolVar` (`self.As Custom Player Controller`)))
        (:`0`
          ;[1 1 1] Checks to see if it is already added to array
          (bind _keys (`BlueprintMapLibrary.Map_Keys` (`self.DestroyedInstances`) :!label _label_3))
          (if (== (`KismetArrayLibrary.Array_Find` _keys _hititem) -1)
            (goto _label)
            (else
              (goto _label_2))))
        (:`1`
          (if (`self.Level1`)
            (set `self.DamageToDo` 5)
            (bind _structout (setmembers `/Game/Dynamic/CustomBPS/FoilageMasters/F_FoilageStruct` :`StructRef` _output :`Health` _returnvalue :!label _label_4))
            (`KismetArrayLibrary.Array_Set` _instances _hititem _structout)
            (if (<= _returnvalue 0)
              (goto _label_3))
            (else
              (`/Game/Dynamic/Widgets/HUD/PlayerHUD_W.WeakTool` (`/Game/Dynamic/Widgets/PlayerMenu/PlayerMenuBase_W.PlayerHUD_W` (`/Game/Dynamic/ThirdPerson/Blueprints/BP_ThirdPersonCharacter.PlayerHud` (`/Game/Dynamic/CustomBPS/CustomPlayerController.As BP Third Person Character` (`self.As Custom Player Controller`)))) :!label _label_5))))
        (:`2`
          (if (`self.Level2`)
            (set `self.DamageToDo` 25)
            (goto _label_4)
            (else
              (goto _label_5))))
        (:`3`
          (if (`self.Level3`)
            (set `self.DamageToDo` 100)
            (goto _label_4)
            (else
              (goto _label_5))))))))

(event `Regrow`
  (bind _destroyedinstances (`self.DestroyedInstances`))
  ;[1 1 1] Tells things to regrow
  (`/Engine/EditorBlueprintResources/StandardMacros.DoOnce` false :!label _label_6
    (:`Completed`
      (bind _keys (`BlueprintMapLibrary.Map_Keys` (`self.DestroyedInstances`)))
      (if (`KismetArrayLibrary.Array_IsValidIndex` _keys)
        (for (_ _array_index) _keys
          (bind _keys_2 (`BlueprintMapLibrary.Map_Keys` _destroyedinstances))
          (bind _values (`BlueprintMapLibrary.Map_Values` _destroyedinstances))
          (if (<= (`KismetMathLibrary.RandomIntegerInRange` 1 100) 33)
            (bind _output (`|GetArrayItem` _keys_2 _array_index))
            (bind _output_2 (`|GetArrayItem` _values _output))
            (bind _returnvalue (+ (.location _output_2) (0.0 0.0 20.0)))
            (bind (_outhit _returnvalue_2) (`KismetSystemLibrary.SphereTraceSingle` :`Start` _returnvalue :`End` _returnvalue :`Radius` 30.0 :`TraceChannel` "TraceTypeQuery1" :`DrawDebugType` "ForDuration"))
            (if (not _returnvalue_2)
              (bind _returnvalue_3 (`self.AddInstance` (`KismetMathLibrary.MakeTransform` (.location _output_2) (struct) (0.1 0.1 0.1)) true))
              (`BlueprintMapLibrary.Map_Remove` (`self.DestroyedInstances`) _output)
              (`KismetArrayLibrary.Array_Add` (`self.Hit Item`) _returnvalue_3)
              (`KismetSystemLibrary.Delay` 0.2)
              (`self.Grow Items`))))
        (goto _label_6 :!via `Reset`)))))

(event `Grow Items`
  (bind _hit_item (`self.Hit Item`))
  ;[1 1 1] Grows things in increments
  (for (_array_element _array_index) (`self.Hit Item`)
    (`KismetArrayLibrary.Array_Remove` _hit_item _array_index)
    (bind _outinstancetransform (`self.GetInstanceTransform` _array_element true))
    (if (not (== (.scale _outinstancetransform) (1.0 1.0 1.0) :`ErrorTolerance` 0.1))
      (`self.RemoveInstance` _array_element)
      (bind _returnvalue (`self.AddInstance` (`KismetMathLibrary.MakeTransform` (.location _outinstancetransform) (.rotation _outinstancetransform) (+ (.scale _outinstancetransform) (0.1 0.1 0.1))) true))
      (`KismetArrayLibrary.Array_Add` _hit_item _returnvalue)
      (`/Engine/EditorBlueprintResources/StandardMacros.IncrementInt` (`self.Iterations`)
        (:`  `
          (`KismetSystemLibrary.Delay` 0.2))))))