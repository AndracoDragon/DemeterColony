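; Game Instance that loads or creates the save object on Init and gathers or restores game state.
; SaveGameFunction copies player and system structs plus NPC and container structs, keyed by actor reference, into SaveGameData; its SaveGameToSlot calls are disconnected.
; LoadGameFunction restores those structs by matching saved keys to level actors.
; Construction parts only reach the instance's ConstructionMap and are not restored; the Ultra_Dynamic_Sky lookup is unused.
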(event `LoadGame`
  (params (SlotName :type String))
  (bind _output_get (set `self.Slot Name Default` SlotName))
  (bind _returnvalue (`GameplayStatics.DoesSaveGameExist` _output_get))
  (if _returnvalue
    (bind _returnvalue_2 (`GameplayStatics.LoadGameFromSlot` (`self.Slot Name Default`)))
    (bind _assave_game_object (cast `/Game/Dynamic/CustomBPS/SaveGameObject` _returnvalue_2))
    (set `self.SaveGameData` _assave_game_object)
    (else
      (bind _returnvalue_3 (`GameplayStatics.CreateSaveGameObject` "/Game/Dynamic/CustomBPS/SaveGameObject.SaveGameObject_C"))
      (set `self.SaveGameData` _returnvalue_3))))

(event `self.ReceiveInit`
  (`self.LoadGame` (`self.Slot Name Default`)))

(event `SaveGame_Event`
  (`self.SaveGame`)
  (`KismetSystemLibrary.Delay` 30.0))

(fn `LoadGameFunction`
  (locals (NPC :type "/Game/Dynamic/NPCs/1ParentNPC1 Object Reference") (FoundNPC :type Boolean) (Container :type "/Game/Dynamic/InventorySystem/1ContainerParent1 Object Reference") (FoundContainer :type Boolean))
  (bind _npc (`local.NPC`))
  (bind _container (`local.Container`))
  (bind _savegamedata (`self.SaveGameData`))
  (`self.SaveGameData`
    (:`then`
      (`|ExecutionSequence`
        (:`then_0`
          (bind _asbp_third_person_character (`/Game/Dynamic/CustomBPS/BlueprintFunctionLibrary.PlayerRefFunction`))
          (set `/Game/Dynamic/ThirdPerson/Blueprints/BP_ThirdPersonCharacter.PlayerStructPBP` (`/Game/Dynamic/CustomBPS/SaveGameObject.PlayerStruct` (`self.SaveGameData`)) _asbp_third_person_character))
        (:`then_1`
          (set `self.SystemStruct` (`/Game/Dynamic/CustomBPS/SaveGameObject.SystemStruct` _savegamedata)))
        (:`then_2`
          (bind _keys (`BlueprintMapLibrary.Map_Keys` (`/Game/Dynamic/CustomBPS/SaveGameObject.NPCStruct` _savegamedata)))
          (for _array_element _keys
            (bind _outactors (`GameplayStatics.GetAllActorsOfClass` "/Game/Dynamic/NPCs/1ParentNPC1.1ParentNPC1_C"))
            (for _array_element_2 _outactors
              (if (== _array_element_2 _array_element)
                (set `local.FoundNPC` true)
                (set `local.NPC` _array_element_2)
                (break)
                (else
                  (set `local.FoundNPC` false))))
            (if (`local.FoundNPC`)
              (set `/Game/Dynamic/NPCs/1ParentNPC1.NPCStruct` (`BlueprintMapLibrary.Map_Find` (`/Game/Dynamic/CustomBPS/SaveGameObject.NPCStruct` (`self.SaveGameData`)) _npc) _npc))))
        (:`then_3`
          (bind _keys_2 (`BlueprintMapLibrary.Map_Keys` (`/Game/Dynamic/CustomBPS/SaveGameObject.ContainerStruct` (`self.SaveGameData`))))
          (for _array_element_3 _keys_2
            (bind _outactors_2 (`GameplayStatics.GetAllActorsOfClass` "/Game/Dynamic/InventorySystem/1ContainerParent1.1ContainerParent1_C"))
            (for _array_element_4 _outactors_2
              (if (== _array_element_4 _array_element_3)
                (set `local.FoundContainer` true)
                (set `local.Container` _array_element_4)
                (break)
                (else
                  (set `local.FoundContainer` false))))
            (if (`local.FoundContainer`)
              (set `/Game/Dynamic/InventorySystem/1ContainerParent1.ContainerStruct` (`BlueprintMapLibrary.Map_Find` (`/Game/Dynamic/CustomBPS/SaveGameObject.ContainerStruct` (`self.SaveGameData`)) _container) _container))))))
    (:`else`)))

(fn `SaveGameFunction`
  (params (SlotName :type String))
  (`|ExecutionSequence`
    (:`then_0`
      (bind _asbp_third_person_character (`/Game/Dynamic/CustomBPS/BlueprintFunctionLibrary.PlayerRefFunction`))
      (`/Game/Dynamic/ThirdPerson/Blueprints/BP_ThirdPersonCharacter.SavingGame` _asbp_third_person_character)
      (set `/Game/Dynamic/CustomBPS/SaveGameObject.PlayerStruct` (`/Game/Dynamic/ThirdPerson/Blueprints/BP_ThirdPersonCharacter.PlayerStructPBP` _asbp_third_person_character) (`self.SaveGameData`)))
    (:`then_1`
      (set `/Game/Dynamic/CustomBPS/SaveGameObject.SystemStruct` (`self.SystemStruct`) (`self.SaveGameData`)))
    (:`then_2`
      (bind _outactors (`GameplayStatics.GetAllActorsOfClass` "/Game/Dynamic/NPCs/1ParentNPC1.1ParentNPC1_C"))
      (for _array_element _outactors
        (`/Game/Dynamic/NPCs/1ParentNPC1.SavingGame` _array_element)
        (`BlueprintMapLibrary.Map_Add` (`/Game/Dynamic/CustomBPS/SaveGameObject.NPCStruct` (`self.SaveGameData`)) _array_element (`/Game/Dynamic/NPCs/1ParentNPC1.NPCStruct` _array_element))))
    (:`then_3`
      (bind _outactors_2 (`GameplayStatics.GetAllActorsOfClass` "/Game/Dynamic/InventorySystem/1ContainerParent1.1ContainerParent1_C"))
      (for _array_element_2 _outactors_2
        (`/Game/Dynamic/InventorySystem/1ContainerParent1.SavingGame` _array_element_2)
        (`BlueprintMapLibrary.Map_Add` (`/Game/Dynamic/CustomBPS/SaveGameObject.ContainerStruct` (`self.SaveGameData`)) _array_element_2 (`/Game/Dynamic/InventorySystem/1ContainerParent1.ContainerStruct` _array_element_2))))
    (:`then_4`
      (bind _outactors_3 (`GameplayStatics.GetAllActorsOfClass` "/Game/Dynamic/CustomBPS/BuildingSystem/BP_ConstructionParent.BP_ConstructionParent_C"))
      (for _array_element_3 _outactors_3
        (`BlueprintMapLibrary.Map_Add` (`self.ConstructionMap`) _array_element_3 (`/Game/Dynamic/CustomBPS/BuildingSystem/BP_ConstructionParent.FConstructionPart` _array_element_3))))
    (:`then_5`
      (`GameplayStatics.GetAllActorsOfClass` "/Game/Dynamic/UltraDynamicSky/Blueprints/Ultra_Dynamic_Sky.Ultra_Dynamic_Sky_C"))))