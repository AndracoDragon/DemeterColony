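; Spline-driven bridge builder that places instanced deck, U-support and support meshes in the construction script.
; Each part's spacing is its mesh bounds on a selectable axis plus an offset, repeated over the spline length with fixed rotation rather than following the tangent.
; Both support types form two offset rows.
; Optional extra supports shift by mesh size, but ignore the loop index, so copies overlap, and use U-support rotation and scale.
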(fn `UserConstructionScript`
  (locals (NumberOfInstanceDeck :type Integer :default 0) (NumberOfInstanceUSupport :type Integer :default 0) (NumberOfInstanceSupport :type Integer :default 0))
  (bind _addextra_ (`self.AddExtra?`))
  (bind _placedmeshsupport (`self.PlacedMeshSupport`))
  (bind _placedmeshdeck (`self.PlacedMeshDeck`))
  (bind _placedmeshusupport (`self.PlacedMeshUSupport`))
  (bind (_returnvalue_min _returnvalue_max) (break `Box` (`StaticMesh.GetBoundingBox` (`self.PlacedMeshSupport`))))
  (bind (_returnvalue_min_2 _returnvalue_max_2) (break `Box` (`StaticMesh.GetBoundingBox` _placedmeshdeck)))
  (bind (_returnvalue_min_3 _returnvalue_max_3) (break `Box` (`StaticMesh.GetBoundingBox` _placedmeshusupport)))
  (bind (_returnvalue_min_4 _returnvalue_max_4) (break `Box` (`StaticMesh.GetBoundingBox` _placedmeshsupport)))
  (bind (_returnvalue_min_5 _returnvalue_max_5) (break `Box` (`StaticMesh.GetBoundingBox` (`self.PlacedMeshSupport`))))
  (bind (_returnvalue_x _returnvalue_y _returnvalue_z) (`KismetMathLibrary.BreakVector` (- _returnvalue_max _returnvalue_min)))
  (bind (_returnvalue_x_2 _returnvalue_y_2 _returnvalue_z_2) (`KismetMathLibrary.BreakVector` (- _returnvalue_max_3 _returnvalue_min_3)))
  (bind (_returnvalue_x_3 _returnvalue_y_3 _returnvalue_z_3) (`KismetMathLibrary.BreakVector` (- _returnvalue_max_4 _returnvalue_min_4)))
  (bind (_returnvalue_x_4 _returnvalue_y_4 _returnvalue_z_4) (`KismetMathLibrary.BreakVector` (- _returnvalue_max_2 _returnvalue_min_2)))
  (bind (_returnvalue_x_5 _returnvalue_y_5 _returnvalue_z_5) (`KismetMathLibrary.BreakVector` (- _returnvalue_max_5 _returnvalue_min_5)))
  (`|ExecutionSequence`
    (:`then_0`
      (`StaticMeshComponent.SetStaticMesh` (`self.ISMDeck`) _placedmeshdeck)
      (set `self.DeckSpacing` (+ (select `byte` (`self.DeckXYZ?`) :`0` _returnvalue_x_4 :`1` _returnvalue_y_4 :`2` _returnvalue_z_4) (`self.DeckOffset`)))
      (bind _output_get (set `local.NumberOfInstanceDeck` (`KismetMathLibrary.FFloor` (/ (`SplineComponent.GetSplineLength` (`self.Spline`)) (`self.DeckSpacing`)))))
      (for _index (range (+ _output_get 1))
        (`InstancedStaticMeshComponent.AddInstance` (`self.ISMDeck`) (`KismetMathLibrary.MakeTransform` (`SplineComponent.GetLocationAtDistanceAlongSpline` (`self.Spline`) (* _index (`self.DeckSpacing`)) "Local") (`self.Deck Rotation`) (`self.Deck Scale`)) false)))
    (:`then_1`
      (`StaticMeshComponent.SetStaticMesh` (`self.ISMUSupport`) _placedmeshusupport)
      (set `self.USupportSpacing` (+ (select `byte` (`self.USupportXYZ?`) :`0` _returnvalue_x_2 :`1` _returnvalue_y_2 :`2` _returnvalue_z_2) (`self.USpportOffset`)))
      (bind _output_get_2 (set `local.NumberOfInstanceUSupport` (`KismetMathLibrary.FFloor` (/ (`SplineComponent.GetSplineLength` (`self.Spline`)) (`self.USupportSpacing`)))))
      (for _index_2 (range (+ _output_get_2 1))
        (`|ExecutionSequence`
          (:`then_0`
            (`InstancedStaticMeshComponent.AddInstance` (`self.ISMUSupport`) (`KismetMathLibrary.MakeTransform` (`KismetMathLibrary.MakeVector` (+ (.x (`SplineComponent.GetLocationAtDistanceAlongSpline` (`self.Spline`) (* _index_2 (`self.USupportSpacing`)) "Local")) (`self.USupportXOffset_1`)) (+ (.y (`SplineComponent.GetLocationAtDistanceAlongSpline` (`self.Spline`) (* _index_2 (`self.USupportSpacing`)) "Local")) (`self.USupportYOffset_1`)) (+ (.z (`SplineComponent.GetLocationAtDistanceAlongSpline` (`self.Spline`) (* _index_2 (`self.USupportSpacing`)) "Local")) (`self.USupportZOffset_1`))) (`self.USpportRotation`) (`self.UsupportScale`)) false))
          (:`then_1`
            (`InstancedStaticMeshComponent.AddInstance` (`self.ISMUSupport`) (`KismetMathLibrary.MakeTransform` (`KismetMathLibrary.MakeVector` (+ (.x (`SplineComponent.GetLocationAtDistanceAlongSpline` (`self.Spline`) (* _index_2 (`self.USupportSpacing`)) "Local")) (`self.USupportXOffset_2`)) (+ (.y (`SplineComponent.GetLocationAtDistanceAlongSpline` (`self.Spline`) (* _index_2 (`self.USupportSpacing`)) "Local")) (`self.USupportYOffset_2`)) (+ (.z (`SplineComponent.GetLocationAtDistanceAlongSpline` (`self.Spline`) (* _index_2 (`self.USupportSpacing`)) "Local")) (`self.USupportZOffset_2`))) (`self.USpportRotation`) (`self.UsupportScale`)) false)))))
    (:`then_2`
      (`StaticMeshComponent.SetStaticMesh` (`self.ISMSupport`) _placedmeshsupport)
      (set `self.SupportSpacing` (+ (select `byte` (`self.SupportXYZ?`) :`0` _returnvalue_x_3 :`1` _returnvalue_y_3 :`2` _returnvalue_z_3) (`self.SupportOffset`)))
      (bind _output_get_3 (set `local.NumberOfInstanceSupport` (`KismetMathLibrary.FFloor` (/ (`SplineComponent.GetSplineLength` (`self.Spline`)) (`self.SupportSpacing`)))))
      (for _index_3 (range (+ _output_get_3 1))
        (`|ExecutionSequence`
          (:`then_0`
            (bind _returnvalue (`KismetMathLibrary.MakeVector` (+ (.x (`SplineComponent.GetLocationAtDistanceAlongSpline` (`self.Spline`) (* _index_3 (`self.SupportSpacing`)) "Local")) (`self.SupportXOffset_1`)) (+ (.y (`SplineComponent.GetLocationAtDistanceAlongSpline` (`self.Spline`) (* _index_3 (`self.SupportSpacing`)) "Local")) (`self.SupportYOffset_1`)) (+ (.z (`SplineComponent.GetLocationAtDistanceAlongSpline` (`self.Spline`) (* _index_3 (`self.SupportSpacing`)) "Local")) (`self.SupportZOffset_1`))))
            (`InstancedStaticMeshComponent.AddInstance` (`self.ISMSupport`) (`KismetMathLibrary.MakeTransform` _returnvalue (`self.SupportRotation`) (`self.SupportScale`)) false)
            (if _addextra_
              (for _ (range (+ (`self.ExtraToAdd`) 1))
                (`InstancedStaticMeshComponent.AddInstance` (`self.ISMSupport`) (`KismetMathLibrary.MakeTransform` (`KismetMathLibrary.MakeVector` (+ (.x (`KismetMathLibrary.MakeVector` (select `bool` (`self.AddOnTheX`) :`true` (+ (.x _returnvalue) _returnvalue_x_5)) (select `bool` (`self.AddOnTheY`) :`true` (+ (.y _returnvalue) _returnvalue_y_5)) (select `bool` (`self.AddOnTheZ`) :`true` (+ (.z _returnvalue) _returnvalue_z_5)))) (`self.SupportXOffset_1`)) (+ (.y (`KismetMathLibrary.MakeVector` (select `bool` (`self.AddOnTheX`) :`true` (+ (.x _returnvalue) _returnvalue_x_5)) (select `bool` (`self.AddOnTheY`) :`true` (+ (.y _returnvalue) _returnvalue_y_5)) (select `bool` (`self.AddOnTheZ`) :`true` (+ (.z _returnvalue) _returnvalue_z_5)))) (`self.SupportYOffset_1`)) (+ (.z (`KismetMathLibrary.MakeVector` (select `bool` (`self.AddOnTheX`) :`true` (+ (.x _returnvalue) _returnvalue_x_5)) (select `bool` (`self.AddOnTheY`) :`true` (+ (.y _returnvalue) _returnvalue_y_5)) (select `bool` (`self.AddOnTheZ`) :`true` (+ (.z _returnvalue) _returnvalue_z_5)))) (`self.SupportZOffset_1`))) (`self.USpportRotation`) (`self.UsupportScale`)) false))))
          (:`then_1`
            (`InstancedStaticMeshComponent.AddInstance` (`self.ISMSupport`) (`KismetMathLibrary.MakeTransform` (`KismetMathLibrary.MakeVector` (+ (.x (`SplineComponent.GetLocationAtDistanceAlongSpline` (`self.Spline`) (* _index_3 (`self.SupportSpacing`)) "Local")) (`self.SupportXOffset_2`)) (+ (.y (`SplineComponent.GetLocationAtDistanceAlongSpline` (`self.Spline`) (* _index_3 (`self.SupportSpacing`)) "Local")) (`self.SupportYOffset_2`)) (+ (.z (`SplineComponent.GetLocationAtDistanceAlongSpline` (`self.Spline`) (* _index_3 (`self.SupportSpacing`)) "Local")) (`self.SupportZOffset_2`))) (`self.SupportRotation`) (`self.SupportScale`)) false)
            (if _addextra_
              (for _ (range (+ (`self.ExtraToAdd`) 1))
                (`InstancedStaticMeshComponent.AddInstance` (`self.ISMSupport`) (`KismetMathLibrary.MakeTransform` (`KismetMathLibrary.MakeVector` (+ (.x (`KismetMathLibrary.MakeVector` (select `bool` (`self.AddOnTheX`) :`true` (+ (.x _returnvalue) _returnvalue_x)) (select `bool` (`self.AddOnTheY`) :`true` (+ (.y _returnvalue) _returnvalue_y)) (select `bool` (`self.AddOnTheZ`) :`true` (+ (.z _returnvalue) _returnvalue_z)))) (`self.SupportXOffset_2`)) (+ (.y (`KismetMathLibrary.MakeVector` (select `bool` (`self.AddOnTheX`) :`true` (+ (.x _returnvalue) _returnvalue_x)) (select `bool` (`self.AddOnTheY`) :`true` (+ (.y _returnvalue) _returnvalue_y)) (select `bool` (`self.AddOnTheZ`) :`true` (+ (.z _returnvalue) _returnvalue_z)))) (`self.SupportYOffset_2`)) (+ (.z (`KismetMathLibrary.MakeVector` (select `bool` (`self.AddOnTheX`) :`true` (+ (.x _returnvalue) _returnvalue_x)) (select `bool` (`self.AddOnTheY`) :`true` (+ (.y _returnvalue) _returnvalue_y)) (select `bool` (`self.AddOnTheZ`) :`true` (+ (.z _returnvalue) _returnvalue_z)))) (`self.SupportZOffset_2`))) (`self.USpportRotation`) (`self.UsupportScale`)) false)))))))))