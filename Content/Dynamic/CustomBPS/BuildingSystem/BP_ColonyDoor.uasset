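; BP_ColonyDoor is a sliding door in the building system that opens on player interaction and closes when the character leaves.
; A box trigger tracks whether BP_ThirdPersonCharacter is in range, gating Interactwith and reversing the Opening timeline on exit.
; The timeline slides the door sideways at a rate derived from OpeningRate, with flags tracking open and closing state.
; LookAt supplies the "Open Door" prompt.
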(event `self.ReceiveBeginPlay`
  (`TimelineComponent.SetPlayRate` (`self.Opening`) (/ 1.0 (`self.OpeningRate`))))

(event `/Game/Dynamic/InventorySystem/I_InteractInterface.InteractWith`
  (params (Player :type "/Game/Dynamic/ThirdPerson/Blueprints/BP_ThirdPersonCharacter Object Reference"))
  (if (and (not (`self.Open`)) (`self.Inrange?`))
    (set `self.Open` true)
    (bind (_direction _openalpha) (`Timeline|Opening` :!label _label)
      (:`Update`
        (`SceneComponent.K2_SetRelativeLocation` (`self.Door`) (`KismetMathLibrary.VLerp` (0.0 0.0 0.0) (0.0 -100.0 0.0) _openalpha) false false))
      (:`Finished`
        (if (`self.Closeing?`)
          (set `self.Open` false)
          (set `self.Closeing?` false)
          (set `self.Moving` false)
          (else
            (set `self.Closeing?` true)))))))

(event `self.Box.OnComponentEndOverlap`
  (params (OverlappedComponent :type "PrimitiveComponent Object Reference") (OtherActor :type "Actor Object Reference") (OtherComp :type "PrimitiveComponent Object Reference") (OtherBodyIndex :type Integer))
  (cast `/Game/Dynamic/ThirdPerson/Blueprints/BP_ThirdPersonCharacter` OtherActor)
  (if (and (`self.Open`) (not (`self.Moving`)))
    (set `self.Closeing?` true)
    (set `self.Inrange?` false)
    (set `self.Moving` true)
    (goto _label :!via `Reverse`)))

(event `self.Box.OnComponentBeginOverlap`
  (params (OverlappedComponent :type "PrimitiveComponent Object Reference") (OtherActor :type "Actor Object Reference") (OtherComp :type "PrimitiveComponent Object Reference") (OtherBodyIndex :type Integer) (bFromSweep :type Boolean) (SweepResult :type "HitResult Structure (by ref)"))
  (cast `/Game/Dynamic/ThirdPerson/Blueprints/BP_ThirdPersonCharacter` OtherActor)
  (set `self.Inrange?` true))

(fn `LookAt`
  (returns (Message :type Text))
  (return "Open Door"))

(fn `UserConstructionScript`)