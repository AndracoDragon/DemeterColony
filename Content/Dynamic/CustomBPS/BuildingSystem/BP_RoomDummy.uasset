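; BP_RoomDummy is the hologram placement preview for a building room, turning red when blocked and green when clear.
; Overlap events and a looping box trace, which flags water, drive the blocked state.
; SetPlace freezes that state, sends hit events to small foliage and plays a timeline that solidifies and enlarges the dummy.
; It then spawns BP_RoomParent at its transform, flattens the dummy vertically and destroys itself.
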(event `self.ReceiveBeginPlay`
  (`PrimitiveComponent.SetMaterial` (`self.RoomDummy`) 0 "/Game/Static/Materials/CustomMats/MI_HologramGreen.MI_HologramGreen")
  (`self.WaterCheckTimer`))

(event `IsBlocked`
  (if (not (`self.SettingInPlace`))
    (`PrimitiveComponent.SetMaterial` (`self.RoomDummy`) 0 "/Game/Static/Materials/CustomMats/MI_HologramRed.MI_HologramRed")
    (set `self.Blocked` true)))

(event `self.RoomDummy.OnComponentBeginOverlap`
  (params (OverlappedComponent :type "PrimitiveComponent Object Reference") (OtherActor :type "Actor Object Reference") (OtherComp :type "PrimitiveComponent Object Reference") (OtherBodyIndex :type Integer) (bFromSweep :type Boolean) (SweepResult :type "HitResult Structure (by ref)"))
  (`self.IsBlocked`))

(event `WaterCheckTimer`
  (`KismetSystemLibrary.K2_SetTimerDelegate` (delegate `WaterCheck`) 0.1 true))

(event `IsUnblocked`
  (if (not (`self.SettingInPlace`))
    (`PrimitiveComponent.SetMaterial` (`self.RoomDummy`) 0 "/Game/Static/Materials/CustomMats/MI_HologramGreen.MI_HologramGreen")
    (set `self.Blocked` false)))

(event `self.RoomDummy.OnComponentEndOverlap`
  (params (OverlappedComponent :type "PrimitiveComponent Object Reference") (OtherActor :type "Actor Object Reference") (OtherComp :type "PrimitiveComponent Object Reference") (OtherBodyIndex :type Integer))
  (if (not (`self.Water`))
    (`self.IsUnblocked`)))

(event `WaterCheck`
  (bind _water (`self.Water`))
  (bind (_outhit _returnvalue) (`KismetSystemLibrary.BoxTraceSingle` (`SceneComponent.K2_GetComponentLocation` (`self.RoomDummy`)) (0.0 0.0 0.0) (250.0 250.0 300.0) (struct) "TraceTypeQuery4"))
  (if _returnvalue
    (if (not _water)
      (`self.IsBlocked`)
      (set `self.Water` true))
    (elif _water
      (`self.IsUnblocked`)
      (set `self.Water` false))))

(event `SetPlace`
  (bind _returnvalue (`self.K2_GetActorLocation`))
  (bind _roomdummy (`self.RoomDummy`))
  (bind _roomdummy_2 (`self.RoomDummy`))
  (set `self.SettingInPlace` true)
  (bind _outhits (`KismetSystemLibrary.BoxTraceMulti` _returnvalue _returnvalue (250.0 250.0 300.0) (struct) "TraceTypeQuery5"))
  (for _array_element _outhits
    (bind _asbp_small_foilage (cast `/Game/Dynamic/CustomBPS/FoilageMasters/BP_SmallFoilage` (`.HitComponent` (`GameplayStatics.BreakHitResult` _array_element))))
    (`/Game/Dynamic/CustomBPS/FoilageMasters/BP_SmallFoilage.Hit Event` _asbp_small_foilage _array_element))
  (bind _returnvalue_2 (`PrimitiveComponent.CreateDynamicMaterialInstance` _roomdummy 0 (`PrimitiveComponent.GetMaterial` _roomdummy 0) "None"))
  (`PrimitiveComponent.SetMaterial` _roomdummy 0 _returnvalue_2)
  (bind (_direction _soldify) (`Timeline|Solidify` :!via `PlayFromStart`)
    (:`Update`
      (`MaterialInstanceDynamic.SetScalarParameterValue` _returnvalue_2 "Opacity" (`KismetMathLibrary.Lerp` 0.5 1.0 _soldify))
      (`SceneComponent.SetWorldScale3D` _roomdummy_2 (`KismetMathLibrary.VLerp` (1.0 1.0 1.0) (1.1 1.1 1.1) _soldify)))
    (:`Finished`
      (`|SpawnActorFromClass` "/Game/Dynamic/CustomBPS/BuildingSystem/BP_RoomParent.BP_RoomParent_C" (`self.GetTransform`) "Undefined" "MultiplyWithRoot" null (struct) null)
      (`KismetSystemLibrary.Delay` 0.5)
      (bind (_direction_2 _shink) (`Timeline|Shrink` :!via `PlayFromStart`)
        (:`Update`
          (`SceneComponent.SetWorldScale3D` _roomdummy_2 (`KismetMathLibrary.VLerp` (1.1 1.1 1.1) (1.1 1.1 0.0) _shink)))
        (:`Finished`
          (`self.K2_DestroyActor`))))))

(fn `UserConstructionScript`)