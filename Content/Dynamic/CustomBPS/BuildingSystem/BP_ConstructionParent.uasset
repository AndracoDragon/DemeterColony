(event `self.ReceiveBeginPlay`
  (bind _mesh (`self.Mesh`))
  (bind _mesh_2 (`self.Mesh`))
  (bind (_fconstructionpart_constructionpart _fconstructionpart_material _fconstructionpart_build _fconstructionpart_notplaced _fconstructionpart_saved _fconstructionpart_transform) (break `/Game/Dynamic/CustomBPS/BuildingSystem/F_ConstructionPart` (`self.FConstructionPart`)))
  (bind _mesh_3 (`self.Mesh`))
  (bind _box (`self.Box`))
  (bind _returnvalue (`MeshComponent.GetMaterials` _mesh))
  (`PrimitiveComponent.SetCollisionEnabled` (`self.Box`) "NoCollision")
  (if _fconstructionpart_saved
    (set `self.Build?` _fconstructionpart_build)
    (set `self.NotPlaced` _fconstructionpart_notplaced)
    (`StaticMeshComponent.SetStaticMesh` _mesh_3 _fconstructionpart_constructionpart)
    (for (_array_element _array_index) _fconstructionpart_material
      (`PrimitiveComponent.SetMaterial` _mesh_3 _array_index _array_element))
    (`self.K2_SetActorTransform` _fconstructionpart_transform)
    (`self.Clear Land`)
    (elif (`self.Placed?`)
      (set `self.NotPlaced` false)
      (set `self.Build?` true)
      (switch `/Game/Dynamic/CustomBPS/BuildingSystem/Enum_ConstructionParts` (`self.ConstructionPart`)
        (:`NewEnumerator0`
          (`self.Clear Land`)))
      (else
        (switch `/Game/Dynamic/CustomBPS/BuildingSystem/Enum_ConstructionParts` (`self.ConstructionPart`)
          (:`NewEnumerator0`
            (`StaticMeshComponent.SetStaticMesh` _mesh_2 "/Game/Static/Patrick_Assets/Meshes/Building_Parents/SM_Parent_Foundation.SM_Parent_Foundation")
            (`BoxComponent.SetBoxExtent` _box (199.0 199.0 75.0) true)
            (`SceneComponent.K2_SetRelativeLocation` _box (0.0 0.0 -9.0) false false)
            (`self.WLTimerStart`)
            (`PrimitiveComponent.SetCollisionEnabled` (`self.Mesh`) "NoCollision" :!label _label)
            (for (_ _array_index_2) _returnvalue
              (`KismetArrayLibrary.Array_Add` (`self.OriMats`) (`PrimitiveComponent.GetMaterial` _mesh _array_index_2)))
            (`KismetSystemLibrary.Delay` 0.2)
            (for (_ _array_index_3) _returnvalue
              (`PrimitiveComponent.SetMaterial` _mesh _array_index_3 "/Game/Static/Materials/CustomMats/MI_HologramGreen.MI_HologramGreen"))
            (`PrimitiveComponent.SetCollisionEnabled` (`self.Box`) "QueryOnly"))
          (:`NewEnumerator1`
            (`StaticMeshComponent.SetStaticMesh` _mesh_2 "/Game/Static/Patrick_Assets/Meshes/Building_Parents/SM_Parent_Wall.SM_Parent_Wall")
            (`BoxComponent.SetBoxExtent` _box (5.0 190.0 121.0) true :!label _label_2)
            (`SceneComponent.K2_SetRelativeLocation` _box (200.0 0.0 191.0) false false))
          (:`NewEnumerator2`
            (`StaticMeshComponent.SetStaticMesh` _mesh_2 "/Game/Static/Patrick_Assets/Meshes/Building_Parents/SM_Parent_Wall_Window.SM_Parent_Wall_Window")
            (goto _label_2))
          (:`NewEnumerator3`
            (`StaticMeshComponent.SetStaticMesh` _mesh_2 "/Game/Static/Patrick_Assets/Meshes/Building_Parents/SM_Parent_Wall_Door.SM_Parent_Wall_Door")
            (goto _label_2))
          (:`NewEnumerator4`
            (`StaticMeshComponent.SetStaticMesh` _mesh_2 "/Game/Static/Meshes/ModularBuildings/PieceModulur/CeilingParent.CeilingParent")
            (`BoxComponent.SetBoxExtent` _box (180.0 180.0 5.0) true)
            (`SceneComponent.K2_SetRelativeLocation` _box (0.0 0.0 316.0) false false)
            (goto _label))
          (:`NewEnumerator5`
            (`StaticMeshComponent.SetStaticMesh` _mesh_2 "/Game/Static/Patrick_Assets/Meshes/Building_Parents/SM_Parent_Stair.SM_Parent_Stair")
            (`BoxComponent.SetBoxExtent` _box (180.0 180.0 120.0) true :!label _label_3)
            (`SceneComponent.K2_SetRelativeLocation` _box (0.0 0.0 195.0) false false)
            (goto _label))
          (:`NewEnumerator6`
            (`StaticMeshComponent.SetStaticMesh` _mesh_2 "/Game/Static/Patrick_Assets/Meshes/Building_Parents/SM_Parent_Stair_Spiral.SM_Parent_Stair_Spiral")
            (goto _label_3)))))))

(event `/Game/Dynamic/CustomBPS/Interfaces/BPI_BuildingInterface.HasFoundation?`
  (params (ImplemetInterface :type Boolean))
  (switch `/Game/Dynamic/CustomBPS/BuildingSystem/Enum_ConstructionParts` (`self.ConstructionPart`)
    (:`NewEnumerator1`
      _)
    (:`NewEnumerator2`
      _)
    (:`NewEnumerator3`
      _)
    (:`NewEnumerator4`
      _)
    (:`NewEnumerator5`
      _)
    (:`NewEnumerator6`
      _))
  (if ImplemetInterface
    (`self.Unblock`)
    (`self.Check for overlap`)
    (else
      (`self.Block`))))

(event `/Game/Dynamic/CustomBPS/Interfaces/BPI_BuildingInterface.DestroyConstruction`
  (bind _mesh (`self.Mesh`))
  (bind _returnvalue (`KismetMaterialLibrary.CreateDynamicMaterialInstance` "/Game/Static/Materials/CustomMats/M_Hologram.M_Hologram"))
  (set `self.BuildGlow` _returnvalue)
  (for (_ _array_index) (`MeshComponent.GetMaterials` _mesh)
    (`PrimitiveComponent.SetMaterial` _mesh _array_index (`self.BuildGlow`))
    (`MaterialInstanceDynamic.SetScalarParameterValue` (`self.BuildGlow`) "Opacity" 1.0))
  (bind (_direction _newtrack_0) (`Timeline|Timeline`)
    (:`Update`
      (`MaterialInstanceDynamic.SetScalarParameterValue` (`self.BuildGlow`) "Opacity" (`KismetMathLibrary.Lerp` 1.0 0.5 _newtrack_0)))
    (:`Finished`
      (`self.K2_DestroyActor`))))

(event `WLTimerStart`
  (bind _returnvalue (`KismetSystemLibrary.K2_SetTimerDelegate` (delegate `Water/landscapecheck`) 0.01 true))
  (set `self.WLTimer` _returnvalue))

(event `Water/landscapecheck`
  (bind _returnvalue (`self.K2_GetActorLocation`))
  (switch `/Game/Dynamic/CustomBPS/BuildingSystem/Enum_ConstructionParts` (`self.ConstructionPart`)
    (:`NewEnumerator0`
      (bind (_outhit _returnvalue_2) (`KismetSystemLibrary.BoxTraceSingle` (+ _returnvalue (0.0 0.0 80.0)) (- _returnvalue (0.0 0.0 80.0)) (199.0 199.0 10.0) (struct) "TraceTypeQuery9"))
      (bind (_bblockinghit _binitialoverlap _time _distance _location _impactpoint _normal _impactnormal _physmat _hitactor) (`GameplayStatics.BreakHitResult` _outhit))
      (cast `Landscape` _hitactor
        (:`then`
          (`self.Unblock` :!label _label_4)
          (`self.Check for overlap`))
        (:`CastFailed`
          (cast `LandscapeProxy` _hitactor
            (:`then`
              (goto _label_4))
            (:`CastFailed`
              (`self.Block`))))))))

(event `/Game/Dynamic/CustomBPS/Interfaces/BPI_BuildingInterface.Rotate`
  (bind (_returnvalue_roll _returnvalue_pitch _returnvalue_yaw) (`KismetMathLibrary.BreakRotator` (`self.K2_GetActorRotation`)))
  (`self.K2_SetActorRotation` (`KismetMathLibrary.MakeRotator` 0.0 0.0 (+ _returnvalue_yaw 90.0)))
  (`self.Check for overlap`))

(event `/Game/Dynamic/CustomBPS/Interfaces/BPI_BuildingInterface.Raise`
  (switch `/Game/Dynamic/CustomBPS/BuildingSystem/Enum_ConstructionParts` (`self.ConstructionPart`)
    (:`NewEnumerator0`
      (`self.K2_SetActorLocation` (+ (`self.K2_GetActorLocation`) (0.0 0.0 10.0))))))

(event `/Game/Dynamic/CustomBPS/Interfaces/BPI_BuildingInterface.Lower`
  (switch `/Game/Dynamic/CustomBPS/BuildingSystem/Enum_ConstructionParts` (`self.ConstructionPart`)
    (:`NewEnumerator0`
      (`self.K2_SetActorLocation` (+ (`self.K2_GetActorLocation`) (0.0 0.0 -10.0))))))

(event `Clear Land`
  (bind _returnvalue (`self.K2_GetActorLocation`))
  (for _ (range 6)
    (bind _outactors (`GameplayStatics.GetAllActorsWithTag` "built"))
    (bind _outhits (`KismetSystemLibrary.BoxTraceMulti` (+ _returnvalue (0.0 0.0 300.0)) (- _returnvalue (0.0 0.0 300.0)) (220.0 220.0 10.0) (struct) "TraceTypeQuery5" false _outactors))
    (for _array_element _outhits
      (bind (_bblockinghit _binitialoverlap _time _distance _location _impactpoint _normal _impactnormal _physmat _hitactor _hitcomponent) (`GameplayStatics.BreakHitResult` _array_element))
      (if (`KismetSystemLibrary.DoesImplementInterface` _hitcomponent "/Game/Dynamic/CustomBPS/Interfaces/BPI_Harvest.BPI_Harvest_C")
        (message `/Game/Dynamic/CustomBPS/Interfaces/BPI_Harvest.HitGrassBuild/Hoe` _hitcomponent _array_element)))))

(event `/Game/Dynamic/CustomBPS/Interfaces/BPI_BuildingInterface.Build`
  (bind _mesh (`self.Mesh`))
  (bind _orimats (`self.OriMats`))
  (if (`self.Build?`)
    (set `self.NotPlaced` false)
    (if (`|EnumEquality` (`self.ConstructionPart`) "NewEnumerator0")
      (`self.Clear Land`))
    (bind _returnvalue (`KismetMaterialLibrary.CreateDynamicMaterialInstance` "/Game/Static/Materials/CustomMats/M_Hologram.M_Hologram"))
    (set `self.BuildGlow` _returnvalue)
    (for (_ _array_index) _orimats
      (`PrimitiveComponent.SetMaterial` (`self.Mesh`) _array_index (`self.BuildGlow`)))
    (bind (_direction _newtrack_0) (`Timeline|IncreaseOpacity` :!via `PlayFromStart`)
      (:`Update`
        (`MaterialInstanceDynamic.SetScalarParameterValue` (`self.BuildGlow`) "Opacity" (`KismetMathLibrary.Lerp` 0.5 1.0 _newtrack_0)))
      (:`Finished`
        (for (_array_element _array_index_2) _orimats
          (`PrimitiveComponent.SetMaterial` (`self.Mesh`) _array_index_2 _array_element))
        (`PrimitiveComponent.SetCollisionEnabled` (`self.Mesh`) "QueryAndPhysics")
        (`KismetSystemLibrary.K2_ClearAndInvalidateTimerHandle` (`self.WLTimer`))
        (setmembers `/Game/Dynamic/CustomBPS/BuildingSystem/F_ConstructionPart` :`StructRef` (`self.FConstructionPart`) :`ConstructionPart` (`StaticMeshComponent.StaticMesh` _mesh) :`Material` (`MeshComponent.GetMaterials` _mesh) :`Build` (`self.Build?`) :`NotPlaced` (`self.NotPlaced`) :`Saved` true :`Transform` (`self.GetTransform`))))))

(event `Check for overlap`
  (bind _box (`self.Box`))
  (for _array_element (`PrimitiveComponent.GetOverlappingActors` _box "BP_ConstructionParent_C")
    (if (`PrimitiveComponent.IsOverlappingActor` _box _array_element)
      (`self.Block` :!label _label_5)
      (else
        (`self.Unblock` :!label _label_6)))))

(event `self.Box.OnComponentBeginOverlap`
  (params (OverlappedComponent :type "PrimitiveComponent Object Reference") (OtherActor :type "Actor Object Reference") (OtherComp :type "PrimitiveComponent Object Reference") (OtherBodyIndex :type Integer) (bFromSweep :type Boolean) (SweepResult :type "HitResult Structure (by ref)"))
  (if (or (`KismetSystemLibrary.DoesImplementInterface` OtherActor "/Game/Dynamic/CustomBPS/Interfaces/BPI_BuildingBlock.BPI_BuildingBlock_C") (`KismetSystemLibrary.DoesImplementInterface` OtherComp "/Game/Dynamic/CustomBPS/Interfaces/BPI_BuildingBlock.BPI_BuildingBlock_C"))
    (goto _label_5)))

(event `Block`
  (if (`self.NotPlaced`)
    (set `self.Build?` false)
    (`PrimitiveComponent.SetMaterial` (`self.Mesh`) 0 "/Game/Static/Materials/CustomMats/MI_HologramRed.MI_HologramRed")))

(event `Unblock`
  (if (`self.NotPlaced`)
    (set `self.Build?` true)
    (`PrimitiveComponent.SetMaterial` (`self.Mesh`) 0 "/Game/Static/Materials/CustomMats/MI_HologramGreen.MI_HologramGreen")))

(event `self.Box.OnComponentEndOverlap`
  (params (OverlappedComponent :type "PrimitiveComponent Object Reference") (OtherActor :type "Actor Object Reference") (OtherComp :type "PrimitiveComponent Object Reference") (OtherBodyIndex :type Integer))
  (if (or (`KismetSystemLibrary.DoesImplementInterface` OtherActor "/Game/Dynamic/CustomBPS/Interfaces/BPI_BuildingBlock.BPI_BuildingBlock_C") (`KismetSystemLibrary.DoesImplementInterface` OtherComp "/Game/Dynamic/CustomBPS/Interfaces/BPI_BuildingBlock.BPI_BuildingBlock_C"))
    (goto _label_6)))

(fn `UserConstructionScript`
  (bind _mesh (`self.Mesh`))
  (if (`self.Placed?`)
    (switch `/Game/Dynamic/CustomBPS/BuildingSystem/Enum_ConstructionParts` (`self.ConstructionPart`)
      (:`NewEnumerator0`
        (`StaticMeshComponent.SetStaticMesh` _mesh "/Game/Static/Meshes/ModularBuildings/PieceModulur/FoundationParent.FoundationParent"))
      (:`NewEnumerator1`
        (`StaticMeshComponent.SetStaticMesh` _mesh "/Game/Static/Meshes/ModularBuildings/PieceModulur/WallParent.WallParent"))
      (:`NewEnumerator2`
        (`StaticMeshComponent.SetStaticMesh` _mesh "/Game/Static/Meshes/ModularBuildings/PieceModulur/WIndowParent.WIndowParent"))
      (:`NewEnumerator3`
        (`StaticMeshComponent.SetStaticMesh` _mesh "/Game/Static/Meshes/ModularBuildings/PieceModulur/DoorParent.DoorParent"))
      (:`NewEnumerator4`
        (`StaticMeshComponent.SetStaticMesh` _mesh "/Game/Static/Meshes/ModularBuildings/PieceModulur/CeilingParent.CeilingParent"))
      (:`NewEnumerator5`
        (`StaticMeshComponent.SetStaticMesh` _mesh "/Game/Static/Meshes/ModularBuildings/PieceModulur/StairParent.StairParent"))
      (:`NewEnumerator6`
        (`StaticMeshComponent.SetStaticMesh` _mesh "/Game/Static/Meshes/ModularBuildings/PieceModulur/SpiralStair.SpiralStair")))))