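; BP_RoomParent is a modular building room configured from RoomInfo, rebuilt on construction and BeginPlay.
; Wall types choose meshes and toggle joiners, stair and floor flags toggle parts, and door flags spawn rotated BP_ColonyDoor actors.
; Adjacent blank walls hide corner pieces, then hidden state drives visibility and collision.
; Themed materials come from DT_BuildingComps by mesh match; the custom colour pass is never run.
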(event `self.ReceiveBeginPlay`
  (`self.SetUpBuildings`))

(fn `BuildingPartArray`
  (returns (Array :type "Array of StaticMeshComponent Object Reference"))
  (return (`|MakeArray` (`self.RoomSkeleton`) (`self.RoomSupport_1`) (`self.Wall_1`) (`self.RoomJoinerSet_1`) (`self.RoomJoinerLeft`) (`self.RoomJoinerRight`) (`self.RoomSupport_2`) (`self.Roof`) (`self.RoomSupport_3`) (`self.RoomSupport_4`) (`self.Floor`) (`self.Stair`) (`self.StairRoof`) (`self.RoomJoinerSet_2`) (`self.RoomJoinerLeft1`) (`self.RoomJoinerRight3`) (`self.Wall_3`) (`self.RoomJoinerSet_3`) (`self.RoomJoinerLeft2`) (`self.RoomJoinerRight2`) (`self.Wall_4`) (`self.RoomJoinerSet_4`) (`self.RoomJoinerLeft3`) (`self.RoomJoinerRight1`))))

(fn `CheckForBlanks`
  (bind (_wall_1 _wall_2 _wall_3 _wall_4) (break `/Game/Dynamic/CustomBPS/BuildingSystem/F_Rooms` (`self.RoomInfo`)))
  (`|ExecutionSequence`
    (:`then_0`
      (if (and (`|EnumEquality` _wall_1 "NewEnumerator0") (`|EnumEquality` _wall_2 "NewEnumerator0"))
        (`SceneComponent.SetHiddenInGame` (`self.RoomJoinerRight`) true false)
        (`SceneComponent.SetHiddenInGame` (`self.RoomJoinerLeft1`) true false)
        (`SceneComponent.SetHiddenInGame` (`self.RoomSupport_1`) true false)))
    (:`then_1`
      (if (and (`|EnumEquality` _wall_2 "NewEnumerator0") (`|EnumEquality` _wall_3 "NewEnumerator0"))
        (`SceneComponent.SetHiddenInGame` (`self.RoomJoinerLeft2`) true false)
        (`SceneComponent.SetHiddenInGame` (`self.RoomJoinerRight3`) true false)
        (`SceneComponent.SetHiddenInGame` (`self.RoomSupport_2`) true false)))
    (:`then_2`
      (if (and (`|EnumEquality` _wall_3 "NewEnumerator0") (`|EnumEquality` _wall_4 "NewEnumerator0"))
        (`SceneComponent.SetHiddenInGame` (`self.RoomJoinerLeft3`) true false)
        (`SceneComponent.SetHiddenInGame` (`self.RoomJoinerRight2`) true false)
        (`SceneComponent.SetHiddenInGame` (`self.RoomSupport_3`) true false)))
    (:`then_3`
      (if (and (`|EnumEquality` _wall_4 "NewEnumerator0") (`|EnumEquality` _wall_1 "NewEnumerator0"))
        (`SceneComponent.SetHiddenInGame` (`self.RoomJoinerLeft`) true false)
        (`SceneComponent.SetHiddenInGame` (`self.RoomJoinerRight1`) true false)
        (`SceneComponent.SetHiddenInGame` (`self.RoomSupport_4`) true false)))
    (:`then_4`
      (if (and (`|EnumEquality` _wall_1 "NewEnumerator0") (`|EnumEquality` _wall_2 "NewEnumerator0") (`|EnumEquality` _wall_3 "NewEnumerator0") (`|EnumEquality` _wall_4 "NewEnumerator0"))
        (`SceneComponent.SetHiddenInGame` (`self.RoomJoinerSet_1`) true true)
        (`SceneComponent.SetHiddenInGame` (`self.RoomJoinerSet_2`) true true)
        (`SceneComponent.SetHiddenInGame` (`self.RoomJoinerSet_3`) true true)
        (`SceneComponent.SetHiddenInGame` (`self.RoomJoinerSet_4`) true true)
        (`SceneComponent.SetHiddenInGame` (`self.RoomSupport_3`) false false)
        (`SceneComponent.SetHiddenInGame` (`self.RoomSupport_2`) false false)
        (`SceneComponent.SetHiddenInGame` (`self.RoomSupport_4`) false false)
        (`SceneComponent.SetHiddenInGame` (`self.RoomSupport_1`) false false)))))

(fn `DoorFunction`
  (params (Door :type "ChildActorComponent Object Reference") (`Usable?` :type Boolean) (Door_1 :type Boolean) (Door_2 :type Boolean) (Door_3 :type Boolean) (Door_4 :type Boolean))
  (bind _returnvalue (`self.K2_GetActorLocation`))
  (`KismetArrayLibrary.Array_Clear` (`self.DoorArray`))
  (`|ExecutionSequence`
    (:`then_0`
      (if Door_1
        (bind _returnvalue_2 (`|SpawnActorFromClass` "/Game/Dynamic/CustomBPS/BuildingSystem/BP_ColonyDoor.BP_ColonyDoor_C" (`KismetMathLibrary.MakeTransform` _returnvalue) "AlwaysSpawn" "MultiplyWithRoot" null 1.5 null))
        (`KismetArrayLibrary.Array_Add` (`self.DoorArray`) _returnvalue_2)))
    (:`then_1`
      (if Door_2
        (bind _returnvalue_3 (`|SpawnActorFromClass` "/Game/Dynamic/CustomBPS/BuildingSystem/BP_ColonyDoor.BP_ColonyDoor_C" (`KismetMathLibrary.MakeTransform` _returnvalue (struct :`Yaw` 90.0)) "AlwaysSpawn" "MultiplyWithRoot" null 1.5 null))
        (`KismetArrayLibrary.Array_Add` (`self.DoorArray`) _returnvalue_3)))
    (:`then_2`
      (if Door_3
        (bind _returnvalue_4 (`|SpawnActorFromClass` "/Game/Dynamic/CustomBPS/BuildingSystem/BP_ColonyDoor.BP_ColonyDoor_C" (`KismetMathLibrary.MakeTransform` _returnvalue (struct :`Yaw` 180.0)) "AlwaysSpawn" "MultiplyWithRoot" null 1.5 null))
        (`KismetArrayLibrary.Array_Add` (`self.DoorArray`) _returnvalue_4)))
    (:`then_3`
      (if Door_4
        (bind _returnvalue_5 (`|SpawnActorFromClass` "/Game/Dynamic/CustomBPS/BuildingSystem/BP_ColonyDoor.BP_ColonyDoor_C" (`KismetMathLibrary.MakeTransform` _returnvalue (struct :`Yaw` 270.0)) "AlwaysSpawn" "MultiplyWithRoot" null 1.5 null))
        (`KismetArrayLibrary.Array_Add` (`self.DoorArray`) _returnvalue_5)))))

(fn `Set Collision`
  (bind _output_get (set `self.StaticMeshArray` (`|MakeArray` (`self.Roof`) (`self.Floor`) (`self.Stair`) (`self.StairRoof`) (`self.Wall_1`) (`self.Wall_2`) (`self.Wall_3`) (`self.Wall_4`) (`self.RoomJoinerSet_1`) (`self.RoomJoinerLeft`) (`self.RoomJoinerRight`) (`self.RoomJoinerSet_2`) (`self.RoomJoinerLeft1`) (`self.RoomJoinerRight1`) (`self.RoomJoinerSet_4`) (`self.RoomJoinerLeft3`) (`self.RoomJoinerRight3`) (`self.RoomJoinerSet_3`) (`self.RoomJoinerLeft2`) (`self.RoomJoinerRight2`) (`self.RoomSupport_1`) (`self.RoomSupport_2`) (`self.RoomSupport_3`) (`self.RoomSupport_4`) (`self.RoomSkeleton`))))
  (for _array_element _output_get
    (bind _bhiddeningame (`SceneComponent.bHiddenInGame` _array_element))
    (`SceneComponent.SetVisibility` _array_element (not _bhiddeningame) false)
    (if _bhiddeningame
      (`PrimitiveComponent.SetCollisionEnabled` _array_element "NoCollision")
      (else
        (`PrimitiveComponent.SetCollisionEnabled` _array_element "QueryAndPhysics")))))

(fn `SetCustomColors`
  (bind _doorarray (`self.DoorArray`))
  (for _array_element (`self.StaticMeshArray`)
    (for (_array_element_2 _array_index) (`MeshComponent.GetMaterialSlotNames` _array_element)
      (bind _returnvalue (`KismetMaterialLibrary.CreateDynamicMaterialInstance` (`PrimitiveComponent.GetMaterial` _array_element _array_index)))
      (`MaterialInstanceDynamic.SetVectorParameterValue` _returnvalue "Color" (`BlueprintMapLibrary.Map_Find` (`.CustomColors_55_3427414E46CFE781CB53F4A85DB5E9C6` (break `/Game/Dynamic/CustomBPS/BuildingSystem/F_Rooms` (`self.RoomInfo`))) _array_element_2))
      (`PrimitiveComponent.SetMaterial` _array_element _array_index _returnvalue)))
  (if (`KismetArrayLibrary.Array_IsValidIndex` _doorarray)
    (for _array_element_3 _doorarray
      (bind _door (`/Game/Dynamic/CustomBPS/BuildingSystem/BP_ColonyDoor.Door` _array_element_3))
      (for (_array_element_4 _array_index_2) (`MeshComponent.GetMaterialSlotNames` _door)
        (bind _returnvalue_2 (`KismetMaterialLibrary.CreateDynamicMaterialInstance` (`PrimitiveComponent.GetMaterial` _door _array_index_2)))
        (`MaterialInstanceDynamic.SetVectorParameterValue` _returnvalue_2 "Color" (`BlueprintMapLibrary.Map_Find` (`.CustomColors_55_3427414E46CFE781CB53F4A85DB5E9C6` (break `/Game/Dynamic/CustomBPS/BuildingSystem/F_Rooms` (`self.RoomInfo`))) _array_element_4))
        (`PrimitiveComponent.SetMaterial` _door _array_index_2 _returnvalue_2)))))

(fn `SetMaterials`
  (bind _doorarray (`self.DoorArray`))
  (bind _output (`|GetArrayItem` (`self.StaticMeshArray`) (`self.VisibleMeshIndex`)))
  (for (_array_element _array_index) (`self.StaticMeshArray`)
    (set `self.VisibleMeshIndex` _array_index)
    (if (not (`SceneComponent.bHiddenInGame` _array_element))
      (bind _outrownames (`DataTableFunctionLibrary.GetDataTableRowNames` "/Game/Dynamic/CustomBPS/BuildingSystem/DT_BuildingComps.DT_BuildingComps"))
      (for _array_element_2 _outrownames
        (bind _returnvalue (`|GetDataTableRow` (`self.Data Table`) _array_element_2)
          (:`then`
            (bind (_staticmesh _materials _buildingtheme) (break `/Game/Dynamic/CustomBPS/BuildingSystem/F_BuildingComps` _returnvalue))
            (if (`|EnumEquality` _buildingtheme (`.BuildingTheme_50_72A738144D33A26715C3F9B29EE0456F` (break `/Game/Dynamic/CustomBPS/BuildingSystem/F_Rooms` (`self.RoomInfo`))))
              (if (== _staticmesh (`StaticMeshComponent.StaticMesh` _output))
                (for (_array_element_3 _array_index_2) _materials
                  (`PrimitiveComponent.SetMaterial` _output _array_index_2 _array_element_3)))))))))
  (if (`KismetArrayLibrary.Array_IsValidIndex` _doorarray)
    (for _array_element_4 _doorarray
      (bind _outrownames_2 (`DataTableFunctionLibrary.GetDataTableRowNames` "/Game/Dynamic/CustomBPS/BuildingSystem/DT_BuildingComps.DT_BuildingComps"))
      (for _array_element_5 _outrownames_2
        (bind _returnvalue_2 (`|GetDataTableRow` (`self.Data Table`) _array_element_5)
          (:`then`
            (bind (_staticmesh_2 _materials_2 _buildingtheme_2) (break `/Game/Dynamic/CustomBPS/BuildingSystem/F_BuildingComps` _returnvalue_2))
            (if (`|EnumEquality` _buildingtheme_2 (`.BuildingTheme_50_72A738144D33A26715C3F9B29EE0456F` (break `/Game/Dynamic/CustomBPS/BuildingSystem/F_Rooms` (`self.RoomInfo`))))
              (bind _door (`/Game/Dynamic/CustomBPS/BuildingSystem/BP_ColonyDoor.Door` _array_element_4))
              (if (== _staticmesh_2 (`StaticMeshComponent.StaticMesh` _door))
                (for (_array_element_6 _array_index_3) _materials_2
                  (`PrimitiveComponent.SetMaterial` _door _array_index_3 _array_element_6))))))))))

(fn `SetUpBuildings`
  (bind (_wall_1 _wall_2 _wall_3 _wall_4 _stairs _upperfloor_ _door_1 _door_2 _door_3 _door_4) (break `/Game/Dynamic/CustomBPS/BuildingSystem/F_Rooms` (`self.RoomInfo`)))
  (`self.SetWallType` _wall_1 (`self.Wall_1`) (`self.RoomJoinerSet_1`))
  (`self.SetWallType` _wall_2 (`self.Wall_2`) (`self.RoomJoinerSet_2`))
  (`self.SetWallType` _wall_3 (`self.Wall_3`) (`self.RoomJoinerSet_3`))
  (`self.SetWallType` _wall_4 (`self.Wall_4`) (`self.RoomJoinerSet_4`))
  (`self.StairsFunction` _stairs _upperfloor_)
  (`self.DoorFunction` null _door_1 _door_1 _door_2 _door_3 _door_4)
  (`self.CheckForBlanks`)
  (`self.Set Collision`)
  (`self.SetMaterials`))

(fn `SetWallType`
  (params (`Wall Typing` :type "/Game/Dynamic/CustomBPS/BuildingSystem/Enum_WallType Enum" :default "NewEnumerator0") (Wall :type "StaticMeshComponent Object Reference") (`Room Joiner Head` :type "SceneComponent Object Reference"))
  (switch `/Game/Dynamic/CustomBPS/BuildingSystem/Enum_WallType` `Wall Typing`
    (:`NewEnumerator0`
      (`SceneComponent.SetHiddenInGame` Wall true false))
    (:`NewEnumerator1`
      (`StaticMeshComponent.SetStaticMesh` Wall "/Game/Static/Meshes/ModularBuildings/Meshes/WallDoor.WallDoor")
      (`SceneComponent.SetHiddenInGame` `Room Joiner Head` true true))
    (:`NewEnumerator2`
      (`StaticMeshComponent.SetStaticMesh` Wall "/Game/Static/Meshes/ModularBuildings/Meshes/WallWindow.WallWindow")
      (`SceneComponent.SetHiddenInGame` `Room Joiner Head` true true))
    (:`NewEnumerator3`
      (`StaticMeshComponent.SetStaticMesh` Wall "/Game/Static/Meshes/ModularBuildings/Meshes/Wall.Wall")
      (`SceneComponent.SetHiddenInGame` `Room Joiner Head` true true)))
  (return))

(fn `StairsFunction`
  (params (`Stairs?` :type Boolean) (`UpperFloor?` :type Boolean))
  (bind _floor (`self.Floor`))
  (bind _roof (`self.Roof`))
  (bind _stair (`self.Stair`))
  (bind _stairroof (`self.StairRoof`))
  (if `Stairs?`
    (`SceneComponent.SetHiddenInGame` _roof true false)
    (`SceneComponent.SetHiddenInGame` _stair false false)
    (`SceneComponent.SetHiddenInGame` _stairroof false false)
    (else
      (`SceneComponent.SetHiddenInGame` _roof false false)
      (`SceneComponent.SetHiddenInGame` _stair true false)
      (`SceneComponent.SetHiddenInGame` _stairroof true false)))
  (if `UpperFloor?`
    (`SceneComponent.SetHiddenInGame` _floor true false)
    (else
      (`SceneComponent.SetHiddenInGame` _floor false false))))

(fn `UserConstructionScript`
  (`self.SetUpBuildings`))