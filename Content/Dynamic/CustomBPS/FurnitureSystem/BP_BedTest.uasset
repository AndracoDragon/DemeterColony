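; BP_BedTest is an interactable bed that prompts "Sleep?" and skips time when used.
; On BeginPlay it finds the Ultra Dynamic Sky actor through its "UDS" tag.
; Interacting fades out the camera and player HUD, disables input, and eases the time of day to a fixed morning hour.
; After a fixed delay it fades back in and restores input.
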(event `self.ReceiveBeginPlay`
  (bind _outactors (`GameplayStatics.GetAllActorsWithTag` "UDS"))
  (bind _asultra_dynamic_sky (cast `/Game/Dynamic/UltraDynamicSky/Blueprints/Ultra_Dynamic_Sky` (`|GetArrayItem` _outactors)))
  (set `self.UDS` _asultra_dynamic_sky))

(event `/Game/Dynamic/InventorySystem/I_InteractInterface.InteractWith`
  (params (Player :type "/Game/Dynamic/ThirdPerson/Blueprints/BP_ThirdPersonCharacter Object Reference"))
  (bind _returnvalue (`GameplayStatics.GetPlayerController` 0))
  (bind _playerhud (`/Game/Dynamic/ThirdPerson/Blueprints/BP_ThirdPersonCharacter.PlayerHud` Player))
  (`PlayerCameraManager.StartCameraFade` :`self` (`GameplayStatics.GetPlayerCameraManager` 0) :`ToAlpha` 1.0 :`Duration` 1.0 :`bHoldWhenFinished` true)
  (`/Game/Dynamic/Widgets/PlayerMenu/PlayerMenuBase_W.Fade` _playerhud)
  (`self.DisableInput` Player _returnvalue)
  (`KismetSystemLibrary.Delay` 1.0)
  (`/Game/Dynamic/UltraDynamicSky/Blueprints/Ultra_Dynamic_Sky.Transition Time of Day` (`self.UDS`) 700.0 10.0 "SinusoidalIn" 5.0 false)
  (`KismetSystemLibrary.Delay` 10.0)
  (`PlayerCameraManager.StartCameraFade` :`self` (`GameplayStatics.GetPlayerCameraManager` 0) :`FromAlpha` 1.0 :`ToAlpha` 0.0 :`Duration` 1.0)
  (`/Game/Dynamic/Widgets/PlayerMenu/PlayerMenuBase_W.FadeIn` _playerhud)
  (`self.EnableInput` Player _returnvalue))

(fn `LookAt`
  (returns (Message :type Text))
  (return "Sleep?"))

(fn `UserConstructionScript`)