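; BP_PortalDrone is a drone actor whose engine and portal materials pulse with an emissive glow.
; On BeginPlay it creates dynamic material instances for two SGDrone material slots and starts a separate timeline for each.
; Each timeline lerps the EmiisivePower parameter between min and max intensities, with play rate set to the inverse of its rate variable.
; A boolean flips on each finish, alternating forward and reverse playback for an endless ping-pong.
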(event `self.ReceiveBeginPlay`
  (bind _sgdrone (`self.SGDrone`))
  (bind _sgdrone_2 (`self.SGDrone`))
  (`|ExecutionSequence`
    (:`then_0`
      (bind _returnvalue (`PrimitiveComponent.CreateDynamicMaterialInstance` _sgdrone_2 3 (`PrimitiveComponent.GetMaterial` _sgdrone 3) "None"))
      (set `self.EngineGlow` _returnvalue)
      (`TimelineComponent.SetPlayRate` (`self.Engine Glow Timelines`) (/ 1.0 (`self.EngineGlowRate`)))
      (`self.EngineGlowEvent`))
    (:`then_1`
      (bind _returnvalue_2 (`PrimitiveComponent.CreateDynamicMaterialInstance` _sgdrone_2 1 (`PrimitiveComponent.GetMaterial` _sgdrone 1) "None"))
      (set `self.PortalGlowVar` _returnvalue_2)
      (`TimelineComponent.SetPlayRate` (`self.PortalGlowTimeline`) (/ 1.0 (`self.PortalGlowRate`)))
      (`self.PortalGlow`))))

(event `EngineGlowEvent`
  (set `self.EngineGowup?` false)
  (bind (_direction _glowtrack) (`Timeline|Engine Glow Timelines` :!label _label)
    (:`Update`
      (`MaterialInstanceDynamic.SetScalarParameterValue` (`self.EngineGlow`) "EmiisivePower" (`KismetMathLibrary.Lerp` (`self.Engine Glow Intensity Min`) (`self.Enigine Glow Intesity Max`) _glowtrack)))
    (:`Finished`
      (if (`self.EngineGowup?`)
        (set `self.EngineGowup?` false)
        (goto _label :!via `PlayFromStart`)
        (else
          (set `self.EngineGowup?` true)
          (goto _label :!via `ReverseFromEnd`))))))

(event `PortalGlow`
  (set `self.PortalGowup?` false)
  (bind (_direction _glowtrack) (`Timeline|PortalGlowTimeline` :!label _label_2)
    (:`Update`
      (`MaterialInstanceDynamic.SetScalarParameterValue` (`self.PortalGlowVar`) "EmiisivePower" (`KismetMathLibrary.Lerp` (`self.PortalGlowIntensityMin`) (`self.PortalGlowIntensityMax`) _glowtrack)))
    (:`Finished`
      (if (`self.PortalGowup?`)
        (set `self.PortalGowup?` false)
        (goto _label_2 :!via `PlayFromStart`)
        (else
          (set `self.PortalGowup?` true)
          (goto _label_2 :!via `ReverseFromEnd`))))))

(fn `UserConstructionScript`)