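; BPC_Compass registers its owning actor on the player's HUD compass with an icon.
; On BeginPlay it waits briefly, casts player 0's character to BP_ThirdPersonCharacter and checks that its PlayerHud is valid.
; It then creates a W_CompassIcon widget from its Icon and owning actor, and adds it to the WCompass overlay panel.
; Registration happens once, with no Tick logic or removal here.
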(event `self.ReceiveBeginPlay`
  (`KismetSystemLibrary.Delay` 0.2)
  (bind _asbp_third_person_character (cast `/Game/Dynamic/ThirdPerson/Blueprints/BP_ThirdPersonCharacter` (`GameplayStatics.GetPlayerCharacter` 0)))
  (bind _playerhud (`/Game/Dynamic/ThirdPerson/Blueprints/BP_ThirdPersonCharacter.PlayerHud` _asbp_third_person_character)
    (:`then`
      (bind _returnvalue (`|CreateWidget` "/Game/Dynamic/Widgets/PlayerMenu/W_CompassIcon.W_CompassIcon_C" null (`self.Icon`) (`self.GetOwner`)))
      (`Overlay.AddChildToOverlay` (`/Game/Dynamic/Widgets/PlayerMenu/W_Compass.OverlayPanel` (`/Game/Dynamic/Widgets/HUD/PlayerHUD_W.W_Compass` (`/Game/Dynamic/Widgets/PlayerMenu/PlayerMenuBase_W.PlayerHUD_W` _playerhud))) _returnvalue))
    (:`else`)))