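; BPC_Dialogue is a component that starts and ends dialogue between the player and an NPC.
; StartDialogue hides the HUD, blends the view to the owning actor and creates W_Dialogue from the NPC's name, dialogue table and player appreciation.
; It then switches to UI-only input with a cursor and triggers the greeting.
; The widget's end event calls EndDialogue, which removes it, forces garbage collection and restores input, view and HUD.
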(event `Start Dialogue`
  (params (Player :type "/Game/Dynamic/ThirdPerson/Blueprints/BP_ThirdPersonCharacter Object Reference") (NPCStruct :type "/Game/Dynamic/NPCs/NPCStruct Structure (by ref)") (NPC :type "/Game/Dynamic/NPCs/1ParentNPC1 Object Reference"))
  (bind ((`Name_2_9E01C8E64A51D1974A001D95A53B4D35` _name) (`PlayerAppreciation_19_41693DE7450B84CBF2F9C78AC0667111` _playerappreciation) (`Working_27_8E4C1D6B40850848180F14A156BD4929` _working) (`NPCDialouge_General_43_C7F5E2B54745F41D0A3B3E8EC389FAF6` _npcdialouge_general)) (break `/Game/Dynamic/NPCs/NPCStruct` NPCStruct))
  (bind _returnvalue (`GameplayStatics.GetPlayerController` 0))
  (`/Game/Dynamic/Widgets/HUD/PlayerHUD_W.HideHudShowDialouge` (`/Game/Dynamic/Widgets/PlayerMenu/PlayerMenuBase_W.PlayerHUD_W` (`/Game/Dynamic/ThirdPerson/Blueprints/BP_ThirdPersonCharacter.PlayerHud` Player)))
  (`PlayerController.SetViewTargetWithBlend` (`PlayerState.GetPlayerController` (`Pawn.PlayerState` Player)) (`self.GetOwner`) 0.0 "VTBlend_Linear" 0.0 false)
  (bind _returnvalue_2 (`|CreateWidget` "/Game/Dynamic/DialogueSystem/W_Dialogue.W_Dialogue_C" null (`KismetTextLibrary.Conv_NameToText` _name) _npcdialouge_general (`KismetMathLibrary.FTrunc` _playerappreciation) (`KismetStringLibrary.Conv_StringToName` (`KismetTextLibrary.Conv_TextToString` (`.PlayerName_2_123B437C448C407C6F4912AFEC5B44BF` (break `/Game/Dynamic/ThirdPerson/Blueprints/PlayerStruct` (`/Game/Dynamic/ThirdPerson/Blueprints/BP_ThirdPersonCharacter.PlayerStructPBP` Player))))) _name NPC Player))
  (set `self.DialogueWidget` _returnvalue_2)
  (add `/Game/Dynamic/DialogueSystem/W_Dialogue.EndDialogue` _returnvalue_2 (delegate `EndDialogue`))
  (`UserWidget.AddToViewport` _returnvalue_2 0)
  (set `PlayerController.bShowMouseCursor` true _returnvalue)
  (`WidgetBlueprintLibrary.SetInputMode_UIOnlyEx` _returnvalue _returnvalue_2)
  (`/Game/Dynamic/DialogueSystem/W_Dialogue.Greeting` _returnvalue_2))

(event `EndDialogue`
  (bind _returnvalue (`GameplayStatics.GetPlayerController` 0))
  (set `PlayerController.bShowMouseCursor` false _returnvalue)
  (`WidgetBlueprintLibrary.SetInputMode_GameOnly` _returnvalue)
  (`Widget.RemoveFromParent` (`self.DialogueWidget`))
  (`KismetSystemLibrary.CollectGarbage`)
  (`PlayerController.SetViewTargetWithBlend` (`PlayerState.GetPlayerController` (`Pawn.PlayerState` (stale `Start Dialogue` Player))) (stale `Start Dialogue` Player) 0.0 "VTBlend_Linear" 0.0 false)
  (`/Game/Dynamic/Widgets/HUD/PlayerHUD_W.HideDialougeShowHud` (`/Game/Dynamic/Widgets/PlayerMenu/PlayerMenuBase_W.PlayerHUD_W` (`/Game/Dynamic/ThirdPerson/Blueprints/BP_ThirdPersonCharacter.PlayerHud` (stale `Start Dialogue` Player)))))